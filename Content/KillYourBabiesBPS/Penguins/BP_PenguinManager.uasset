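; Penguin manager that spawns penguins in the level, tracks those the player carries, and decides seal target priority.
; BeginPlay shuffles spawn points and spawns penguins at random free ones, recorded in a point-to-penguin map.
; Tick checks the character's penguin mesh visibility top-down to set ready flags, throw start location and Niagara effects, then updates BP_Peixes1.
; It also flags dropped-penguin priority when one is at least as near the seal as the player.
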(event `self.ReceiveTick`
  (params (DeltaSeconds :type "Float (single-precision)"))
  (`self.CheckDistance`)
  (`GameplayStatics.GetActorOfClass` "/Game/KillYourBabiesBPS/BPS_Foca/FocaTentativa.FocaTentativa_C")
  (bind _returnvalue (`GameplayStatics.GetActorOfClass` "/Game/KillYourBabiesBPS/BP_PLayer/BP_ThirdPersonCharacterKYB.BP_ThirdPersonCharacterKYB_C"))
  (bind _penguin4 (`/Game/KillYourBabiesBPS/BP_PLayer/BP_ThirdPersonCharacterKYB.Penguin4` _returnvalue))
  (if (`SceneComponent.IsVisible` _penguin4)
    (set `/Game/KillYourBabiesBPS/BP_PLayer/BP_ThirdPersonCharacterKYB.Has4PenguinReady` true _returnvalue)
    (set `/Game/KillYourBabiesBPS/BP_PLayer/BP_ThirdPersonCharacterKYB.Has3PenguinReady` false _returnvalue)
    (set `/Game/KillYourBabiesBPS/BP_PLayer/BP_ThirdPersonCharacterKYB.Has2PenguinReady` false _returnvalue)
    (set `/Game/KillYourBabiesBPS/BP_PLayer/BP_ThirdPersonCharacterKYB.Has1PenguinReady` false _returnvalue)
    (set `/Game/KillYourBabiesBPS/BP_PLayer/BP_ThirdPersonCharacterKYB.Has0PenguinReady` false _returnvalue)
    (set `/Game/KillYourBabiesBPS/BP_PLayer/BP_ThirdPersonCharacterKYB.PenguinStart` (`SceneComponent.K2_GetComponentLocation` _penguin4) _returnvalue)
    (bind _returnvalue_2 (`GameplayStatics.GetActorOfClass` "/Game/KillYourBabiesBPS/Peixes/Os_3_Peixes/BP_Peixes1.BP_Peixes1_C"))
    (`/Game/KillYourBabiesBPS/Peixes/Os_3_Peixes/BP_Peixes1.PeixeUpdate` _returnvalue_2)
    (bind _niagara4 (`/Game/KillYourBabiesBPS/BP_PLayer/BP_ThirdPersonCharacterKYB.Niagara4` _returnvalue))
    (`ActorComponent.Activate` _niagara4 false)
    (else
      (bind _penguin3 (`/Game/KillYourBabiesBPS/BP_PLayer/BP_ThirdPersonCharacterKYB.Penguin3` _returnvalue))
      (if (`SceneComponent.IsVisible` _penguin3)
        (set `/Game/KillYourBabiesBPS/BP_PLayer/BP_ThirdPersonCharacterKYB.Has4PenguinReady` false _returnvalue)
        (set `/Game/KillYourBabiesBPS/BP_PLayer/BP_ThirdPersonCharacterKYB.Has3PenguinReady` true _returnvalue)
        (set `/Game/KillYourBabiesBPS/BP_PLayer/BP_ThirdPersonCharacterKYB.Has2PenguinReady` false _returnvalue)
        (set `/Game/KillYourBabiesBPS/BP_PLayer/BP_ThirdPersonCharacterKYB.Has1PenguinReady` false _returnvalue)
        (set `/Game/KillYourBabiesBPS/BP_PLayer/BP_ThirdPersonCharacterKYB.Has0PenguinReady` false _returnvalue)
        (set `/Game/KillYourBabiesBPS/BP_PLayer/BP_ThirdPersonCharacterKYB.PenguinStart` (`SceneComponent.K2_GetComponentLocation` _penguin3) _returnvalue)
        (bind _returnvalue_3 (`GameplayStatics.GetActorOfClass` "/Game/KillYourBabiesBPS/Peixes/Os_3_Peixes/BP_Peixes1.BP_Peixes1_C"))
        (`/Game/KillYourBabiesBPS/Peixes/Os_3_Peixes/BP_Peixes1.PeixeUpdate` _returnvalue_3)
        (bind _niagara3 (`/Game/KillYourBabiesBPS/BP_PLayer/BP_ThirdPersonCharacterKYB.Niagara3` _returnvalue))
        (`ActorComponent.Activate` _niagara3 false)
        (`ActorComponent.Deactivate` _niagara4)
        (else
          (bind _penguin2 (`/Game/KillYourBabiesBPS/BP_PLayer/BP_ThirdPersonCharacterKYB.Penguin2` _returnvalue))
          (if (`SceneComponent.IsVisible` _penguin2)
            (set `/Game/KillYourBabiesBPS/BP_PLayer/BP_ThirdPersonCharacterKYB.Has4PenguinReady` false _returnvalue)
            (set `/Game/KillYourBabiesBPS/BP_PLayer/BP_ThirdPersonCharacterKYB.Has3PenguinReady` false _returnvalue)
            (set `/Game/KillYourBabiesBPS/BP_PLayer/BP_ThirdPersonCharacterKYB.Has2PenguinReady` true _returnvalue)
            (set `/Game/KillYourBabiesBPS/BP_PLayer/BP_ThirdPersonCharacterKYB.Has1PenguinReady` false _returnvalue)
            (set `/Game/KillYourBabiesBPS/BP_PLayer/BP_ThirdPersonCharacterKYB.Has0PenguinReady` false _returnvalue)
            (set `/Game/KillYourBabiesBPS/BP_PLayer/BP_ThirdPersonCharacterKYB.PenguinStart` (`SceneComponent.K2_GetComponentLocation` _penguin2) _returnvalue)
            (bind _returnvalue_4 (`GameplayStatics.GetActorOfClass` "/Game/KillYourBabiesBPS/Peixes/Os_3_Peixes/BP_Peixes1.BP_Peixes1_C"))
            (`/Game/KillYourBabiesBPS/Peixes/Os_3_Peixes/BP_Peixes1.PeixeUpdate` _returnvalue_4)
            (bind _niagara2 (`/Game/KillYourBabiesBPS/BP_PLayer/BP_ThirdPersonCharacterKYB.Niagara2` _returnvalue))
            (`ActorComponent.Activate` _niagara2 false)
            (`ActorComponent.Deactivate` _niagara3)
            (else
              (bind _penguin1 (`/Game/KillYourBabiesBPS/BP_PLayer/BP_ThirdPersonCharacterKYB.Penguin1` _returnvalue))
              (if (`SceneComponent.IsVisible` _penguin1)
                (set `/Game/KillYourBabiesBPS/BP_PLayer/BP_ThirdPersonCharacterKYB.Has4PenguinReady` false _returnvalue)
                (set `/Game/KillYourBabiesBPS/BP_PLayer/BP_ThirdPersonCharacterKYB.Has3PenguinReady` false _returnvalue)
                (set `/Game/KillYourBabiesBPS/BP_PLayer/BP_ThirdPersonCharacterKYB.Has2PenguinReady` false _returnvalue)
                (set `/Game/KillYourBabiesBPS/BP_PLayer/BP_ThirdPersonCharacterKYB.Has1PenguinReady` true _returnvalue)
                (set `/Game/KillYourBabiesBPS/BP_PLayer/BP_ThirdPersonCharacterKYB.Has0PenguinReady` false _returnvalue)
                (else
                  (set `/Game/KillYourBabiesBPS/BP_PLayer/BP_ThirdPersonCharacterKYB.Has4PenguinReady` false _returnvalue)
                  (set `/Game/KillYourBabiesBPS/BP_PLayer/BP_ThirdPersonCharacterKYB.Has3PenguinReady` false _returnvalue)
                  (set `/Game/KillYourBabiesBPS/BP_PLayer/BP_ThirdPersonCharacterKYB.Has2PenguinReady` false _returnvalue)
                  (set `/Game/KillYourBabiesBPS/BP_PLayer/BP_ThirdPersonCharacterKYB.Has1PenguinReady` false _returnvalue)
                  (set `/Game/KillYourBabiesBPS/BP_PLayer/BP_ThirdPersonCharacterKYB.Has0PenguinReady` true _returnvalue)
                  (bind _niagara1 (`/Game/KillYourBabiesBPS/BP_PLayer/BP_ThirdPersonCharacterKYB.Niagara1` _returnvalue))
                  (`ActorComponent.Deactivate` _niagara1)))
              (set `/Game/KillYourBabiesBPS/BP_PLayer/BP_ThirdPersonCharacterKYB.PenguinStart` (`SceneComponent.K2_GetComponentLocation` _penguin1) _returnvalue)
              (bind _returnvalue_5 (`GameplayStatics.GetActorOfClass` "/Game/KillYourBabiesBPS/Peixes/Os_3_Peixes/BP_Peixes1.BP_Peixes1_C"))
              (`/Game/KillYourBabiesBPS/Peixes/Os_3_Peixes/BP_Peixes1.PeixeUpdate` _returnvalue_5)
              (`ActorComponent.Activate` _niagara1 false)
              (`ActorComponent.Deactivate` _niagara2))))))))

(event `CheckDistance`
  (bind _returnvalue (`GameplayStatics.GetActorOfClass` "/Game/KillYourBabiesBPS/Penguins/PenguinSpots/Penguin_Dropped.Penguin_Dropped_C"))
  (`/Engine/EditorBlueprintResources/StandardMacros.IsValid` _returnvalue
    (:`Is Valid`
      (`KismetSystemLibrary.PrintString` "CheckingDistance")
      (bind _returnvalue_2 (`GameplayStatics.GetActorOfClass` "/Game/KillYourBabiesBPS/BPS_Foca/FocaNavPointFollow.FocaNavPointFollow_C"))
      (bind _returnvalue_3 (`GameplayStatics.GetActorOfClass` "/Game/KillYourBabiesBPS/BP_PLayer/BP_ThirdPersonCharacterKYB.BP_ThirdPersonCharacterKYB_C"))
      (bind _returnvalue_4 (`GameplayStatics.GetActorOfClass` "/Game/KillYourBabiesBPS/Penguins/PenguinSpots/Penguin_Dropped.Penguin_Dropped_C"))
      (bind _returnvalue_5 (`SceneComponent.K2_GetComponentLocation` (`Character.CapsuleComponent` _returnvalue_2)))
      (set `self.DistancePlayerToSeal` (`KismetMathLibrary.Vector_Distance` _returnvalue_5 (`SceneComponent.K2_GetComponentLocation` (`Character.CapsuleComponent` _returnvalue_3))))
      (set `self.DistanceDroppedPenguinToSeal` (`KismetMathLibrary.Vector_Distance` (`SceneComponent.K2_GetComponentLocation` (`/Game/KillYourBabiesBPS/Penguins/PenguinSpots/Penguin_Dropped.Capsule` _returnvalue_4)) _returnvalue_5))
      (if (<= (`self.DistanceDroppedPenguinToSeal`) (`self.DistancePlayerToSeal`))
        (set `self.DroppedPenguinPriority` true)
        (`GameplayStatics.GetActorOfClass` "/Game/KillYourBabiesBPS/BPS_Foca/FocaNavPointFollow.FocaNavPointFollow_C")
        (`KismetSystemLibrary.PrintString` "PertoPinguimLargado")
        (else
          (set `self.DroppedPenguinPriority` false)
          (`KismetSystemLibrary.PrintString` "PertoPlayer"))))
    (:`Is Not Valid`
      (set `self.DroppedPenguinPriority` false))))

(event `self.ReceiveBeginPlay`
  (bind _outactors (`GameplayStatics.GetAllActorsOfClass` "/Game/KillYourBabiesBPS/Penguins/BP_PenguinSpawnPoint.BP_PenguinSpawnPoint_C"))
  (bind _output_get (set `self.PenguinSpawnPointsArray` _outactors))
  (`KismetArrayLibrary.Array_Shuffle` _output_get)
  (for _ (range 3)
    (`self.SpawnPenguinAtPoint`)))

(fn `SpawnPenguinAtPoint`
  (locals (FreePenguinPoints :type "Array of /Game/KillYourBabiesBPS/Penguins/BP_PenguinSpawnPoint Object Reference"))
  (bind _freepenguinpoints (`local.FreePenguinPoints`))
  (bind _returnvalue (`KismetArrayLibrary.Array_Length` _freepenguinpoints))
  (for _array_element (`self.PenguinSpawnPointsArray`)
    (if (not (`BlueprintMapLibrary.Map_Contains` (`self.ActivePenguinMap`) _array_element))
      (`KismetArrayLibrary.Array_Add` _freepenguinpoints _array_element)))
  (`KismetSystemLibrary.PrintString` (`KismetStringLibrary.Conv_IntToString` _returnvalue))
  (if (> _returnvalue 0)
    (bind _output_get (set `self.SelectedPenguinPoint` (`|GetArrayItem` _freepenguinpoints (`KismetMathLibrary.RandomIntegerInRange` 0 (+ _returnvalue -1)))))
    (bind _returnvalue_2 (`|SpawnActorFromClass` "/Game/KillYourBabiesBPS/Penguins/PenguinSpots/Penguin_Spawned.Penguin_Spawned_C" (`KismetMathLibrary.MakeTransform` (`self.K2_GetActorLocation` _output_get) (`self.K2_GetActorRotation` _output_get)) "Undefined" "MultiplyWithRoot" null null))
    (set `/Game/KillYourBabiesBPS/Penguins/PenguinSpots/Penguin_Spawned.ThisSpawnPoint` _output_get _returnvalue_2)
    (`BlueprintMapLibrary.Map_Add` (`self.ActivePenguinMap`) _output_get _returnvalue_2)))

(fn `UserConstructionScript`)