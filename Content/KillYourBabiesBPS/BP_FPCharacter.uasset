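; BP_FPCharacter is an underwater player character with sprint swimming, oxygen and stamina.
; Shift runs a retriggerable-delay loop that drains both resources and raises swim speed, with timelines animating camera FOV; W similarly drives movement along camera forward.
; Tick drains oxygen, regenerates stamina below the oxygen level, varies Niagara bubbles by sprint state and maps camera depth to exposure compensation.
; Enter refills both resources, and BeginPlay creates the stamina widget.
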(event `Key|Enter`
  (params (Key :type "Key Structure"))
  (:`Pressed`
    (set `self.Oxigen` 100.0)
    (set `self.Stamina` 100.0)))

(event `self.ReceiveBeginPlay`
  (bind _returnvalue (`|CreateWidget` "/Game/UI/UI_Stamina.UI_Stamina_C" (`GameplayStatics.GetPlayerController` 0)))
  (`UserWidget.AddToViewport` _returnvalue 0))

(event `Key|LeftShift`
  (params (Key :type "Key Structure"))
  (bind _charactermovement (`self.CharacterMovement`))
  (:`Pressed`
    (set `self.isRunning` true)
    (if (<= (`self.Stamina`) 0.1) :!label _label
      (set `self.isRunning` false :!label _label_2)
      (bind _returnvalue (`BlueprintCameraPoseFunctionLibrary.MakeCameraPoseFromCameraComponent` (`self.FollowCamera`)))
      (if (not (< (`BlueprintCameraPoseFunctionLibrary.GetFieldOfView` _returnvalue) 105.0))
        (bind (_direction _fovtrack) (`Timeline|Timeline_0` :!via `ReverseFromEnd`)
          (:`Update`
            (bind _returnvalue_2 (`BlueprintCameraPoseFunctionLibrary.MakeCameraPoseFromCameraComponent` (`self.FollowCamera`)))
            (`CameraComponent.SetFieldOfView` (`self.FollowCamera`) (`KismetMathLibrary.Lerp` 90.0 (`BlueprintCameraPoseFunctionLibrary.GetFieldOfView` _returnvalue_2) _fovtrack)))))
      (set `CharacterMovementComponent.MaxSwimSpeed` 1000.0 _charactermovement)
      (else
        (bind _returnvalue_3 (`BlueprintCameraPoseFunctionLibrary.MakeCameraPoseFromCameraComponent` (`self.FollowCamera`)))
        (if (== (`BlueprintCameraPoseFunctionLibrary.GetFieldOfView` _returnvalue_3) 105.0)
          (set `CharacterMovementComponent.MaxSwimSpeed` 2700.0 _charactermovement :!label _label_3)
          (`KismetSystemLibrary.RetriggerableDelay` 0.02)
          (`self.UseStamina`)
          (if (`self.isRunning`)
            (goto _label))
          (else
            (`self.UseStamina`)
            (bind (_direction_2 _fov) (`Timeline|Timeline` :!via `PlayFromStart`)
              (:`Update`
                (if (not (`PlayerController.IsInputKeyDown` (`GameplayStatics.GetPlayerController` 0) "LeftShift"))
                  (bind _returnvalue_4 (`BlueprintCameraPoseFunctionLibrary.MakeCameraPoseFromCameraComponent` (`self.FollowCamera`)))
                  (bind (_direction_3 _fovtrack_2) (`Timeline|Timeline_2` :!via `ReverseFromEnd`)
                    (:`Update`
                      (`CameraComponent.SetFieldOfView` (`self.FollowCamera`) (`KismetMathLibrary.Lerp` 90.0 (`BlueprintCameraPoseFunctionLibrary.GetFieldOfView` _returnvalue_4) _fovtrack_2))))
                  (else
                    (`CameraComponent.SetFieldOfView` (`self.FollowCamera`) (`KismetMathLibrary.Lerp` 90.0 105.0 _fov))
                    (goto _label_3))))))))))
  (:`Released`
    (goto _label_2)))

(event `UseStamina`
  (set `self.Stamina` (- (`self.Stamina`) 0.7))
  (set `self.Oxigen` (- (`self.Oxigen`) 0.15)))

(event `DecreaseOxigen`
  (set `self.Oxigen` (- (`self.Oxigen`) 0.008))
  (if (>= (`self.Stamina`) (`self.Oxigen`))
    (set `self.Stamina` (- (`self.Stamina`) 0.007))))

(event `Key|W`
  (params (Key :type "Key Structure"))
  (:`Pressed`
    (bind _output_get (set `self.IsPressingW` true))
    (if _output_get :!label _label_4
      (`KismetSystemLibrary.RetriggerableDelay` 0.02)
      (`self.AddMovementInput` (`KismetMathLibrary.GetForwardVector` (`SceneComponent.K2_GetComponentRotation` (`self.FollowCamera`))) 500.0)
      (goto _label_4)
      (else
        (set `self.IsPressingW` false :!label _label_5))))
  (:`Released`
    (goto _label_5)))

(event `IncreaseStamina`
  (set `self.Stamina` (+ (`self.Stamina`) 0.1)))

(event `self.ReceiveTick`
  (params (DeltaSeconds :type "Float (single-precision)"))
  (`self.BubblesSwitcher`)
  (`self.ExposureFunction`)
  (if (<= (`self.Oxigen`) 0.0)
    (`KismetSystemLibrary.PrintString` "SprintNoMore")
    (else
      (`self.DecreaseOxigen`)
      (if (not (> (`self.Stamina`) (`self.Oxigen`)))
        (`self.IncreaseStamina`)))))

(event `BubblesSwitcher`
  (if (`self.isRunning`)
    (`NiagaraComponent.SetVariableFloat` (`self.Niagara`) "Sprinting" (`KismetMathLibrary.RandomFloatInRange` 15.0 25.0))
    (`KismetSystemLibrary.RetriggerableDelay` 2.0)
    (else
      (`NiagaraComponent.SetVariableFloat` (`self.Niagara`) "Sprinting" (`KismetMathLibrary.RandomFloatInRange` 2.0 8.0))
      (`KismetSystemLibrary.RetriggerableDelay` 2.0))))

(fn `ExposureFunction`
  (bind (_returnvalue_x _returnvalue_y _returnvalue_z) (`KismetMathLibrary.BreakVector` (`SceneComponent.K2_GetComponentLocation` (`self.FollowCamera`))))
  (if true
    (setmembers `PostProcessSettings` :`StructRef` (`PostProcessComponent.Settings` (`self.PostProcess`)) :`AutoExposureBias` (`KismetMathLibrary.MapRangeClamped` _returnvalue_z 1000.0 -24900.0))))

(fn `UserConstructionScript`)