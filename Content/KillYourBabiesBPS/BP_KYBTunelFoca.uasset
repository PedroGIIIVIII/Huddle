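; Swimming seal (Foca) AI character that rides a dynamic spline, with unused patrol and chase logic.
; Tick places the seal mesh along the first BP_DynamicSpline with optional looping, but passes zero delta time, so distance never advances by speed.
; Self-repeating AIMoveTo events patrol four points or chase the player at higher swim speed.
; Their view-cone and distance detection check is disconnected, so neither starts here.
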(event `self.ReceiveTick`
  (params (DeltaSeconds :type "Float (single-precision)"))
  (`self.FollowingSpline` 0.0))

(event `FocaFollow`
  (set `CharacterMovementComponent.MaxSwimSpeed` 1200.0 (`self.CharacterMovement`))
  (`|AIMoveTo` self (`NavigationSystemV1.K2_ProjectPointToNavigation` (`self.K2_GetActorLocation` (`GameplayStatics.GetPlayerCharacter` 0)) null null (1500.0 1500.0 1500.0)) null
    (:`OnSuccess`
      (`self.FocaFollow`))))

(event `FollowingSpline`
  (params (DeltaSeconds :type "Float (single-precision)"))
  (bind _returnvalue (`GameplayStatics.GetActorOfClass` "/Game/KillYourBabiesBPS/BP_DynamicSpline.BP_DynamicSpline_C"))
  (bind _asbp_dynamic_spline (cast `/Game/KillYourBabiesBPS/BP_DynamicSpline` _returnvalue))
  (set `self.DistanceAlongSpline` (+ (* DeltaSeconds (`self.SplineSpeed`)) (`self.DistanceAlongSpline`)))
  (bind _spline (`/Game/KillYourBabiesBPS/BP_DynamicSpline.Spline` _asbp_dynamic_spline))
  (bind _returnvalue_2 (`SplineComponent.GetTransformAtDistanceAlongSpline` _spline (`self.DistanceAlongSpline`) "Local" false))
  (`SceneComponent.K2_SetRelativeTransform` (`self.Foca`) (`KismetMathLibrary.MakeTransform` (`KismetMathLibrary.MakeVector` (.x (.location _returnvalue_2)) (+ (.y (.location _returnvalue_2)) -89.0) (.z (.location _returnvalue_2))) (`KismetMathLibrary.MakeRotator` (.roll (.rotation _returnvalue_2)) (.pitch (.rotation _returnvalue_2)) (.yaw (.rotation _returnvalue_2))) (`SceneComponent.RelativeScale3D` (`self.Foca`))) false false)
  (if (`self.Loop`)
    (if (> (`self.DistanceAlongSpline`) (`SplineComponent.GetSplineLength` _spline))
      (set `self.DistanceAlongSpline` 0.0))))

(event `FocaPatrol`
  (set `CharacterMovementComponent.MaxSwimSpeed` 600.0 (`self.CharacterMovement`))
  (`|AIMoveTo` self (`|GetArrayItem` (`self.PatrolLocation`) (`self.Locations`)) null
    (:`OnSuccess`
      (`self.FocaPatrol`)
      (`/Engine/EditorBlueprintResources/StandardMacros.IncrementInt` (`self.Locations`)
        (:`  `
          (if (== (`self.Locations`) 4)
            (set `self.Locations` 0)))))))

(fn `UserConstructionScript`)