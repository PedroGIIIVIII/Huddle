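; BP_LimitPeixes is an actor that caps the player's fish count (Peixes) according to the penguin-ready stage.
; Every Tick it finds the player character by class and clamps Peixes to a limit that rises with each stage.
; When clamping, it calls PeixeUpdate on BP_Peixes1.
; At the first stage, if a TutorialManager exists, it also prints debug text and requests a UI hint unless the second trigger box has fired.
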(event `self.ReceiveTick`
  (params (DeltaSeconds :type "Float (single-precision)"))
  (bind _returnvalue (`GameplayStatics.GetActorOfClass` "/Game/KillYourBabiesBPS/BP_PLayer/BP_ThirdPersonCharacterKYB.BP_ThirdPersonCharacterKYB_C"))
  (bind _returnvalue_2 (`GameplayStatics.GetActorOfClass` "/Game/KillYourBabiesBPS/Peixes/Os_3_Peixes/BP_Peixes1.BP_Peixes1_C"))
  (bind _peixes (`/Game/KillYourBabiesBPS/BP_PLayer/BP_ThirdPersonCharacterKYB.Peixes` _returnvalue))
  (if (and (`/Game/KillYourBabiesBPS/BP_PLayer/BP_ThirdPersonCharacterKYB.Has0PenguinReady` _returnvalue) (> _peixes 5.0))
    (set `/Game/KillYourBabiesBPS/BP_PLayer/BP_ThirdPersonCharacterKYB.Peixes` 5.0 _returnvalue)
    (bind _returnvalue_3 (`GameplayStatics.GetActorOfClass` "/Game/KillYourBabiesBPS/Tutorial/TutorialManager.TutorialManager_C"))
    (`/Engine/EditorBlueprintResources/StandardMacros.IsValid` _returnvalue_3
      (:`Is Valid`
        (`/Game/KillYourBabiesBPS/Peixes/Os_3_Peixes/BP_Peixes1.PeixeUpdate` _returnvalue_2)
        (`KismetSystemLibrary.PrintString` "MMMMMMMMMMMMMMMMMMMMMMMMMMMMMMMMMMMMMMMMMMMMMMMMMMMMMMMMMMMMMMMMMMMMMMMMMMMMMMMMMMMMMMMMMMMMMMMMM")
        (bind _returnvalue_4 (`GameplayStatics.GetActorOfClass` "/Game/KillYourBabiesBPS/Tutorial/2ºTriggerBox_Blueprint.2ºTriggerBox_Blueprint_C"))
        (if (not (`/Game/KillYourBabiesBPS/Tutorial/2ºTriggerBox_Blueprint.2º_Trigger` _returnvalue_4))
          (`/Game/KillYourBabiesBPS/Tutorial/TutorialManager.GetUIHint` _returnvalue_3)))
      (:`Is Not Valid`
        (`/Game/KillYourBabiesBPS/Peixes/Os_3_Peixes/BP_Peixes1.PeixeUpdate` _returnvalue_2)))
    (elif (and (`/Game/KillYourBabiesBPS/BP_PLayer/BP_ThirdPersonCharacterKYB.Has1PenguinReady` _returnvalue) (> _peixes 10.0))
      (set `/Game/KillYourBabiesBPS/BP_PLayer/BP_ThirdPersonCharacterKYB.Peixes` 10.0 _returnvalue)
      (`/Game/KillYourBabiesBPS/Peixes/Os_3_Peixes/BP_Peixes1.PeixeUpdate` _returnvalue_2)
      (elif (and (`/Game/KillYourBabiesBPS/BP_PLayer/BP_ThirdPersonCharacterKYB.Has2PenguinReady` _returnvalue) (> _peixes 15.0))
        (set `/Game/KillYourBabiesBPS/BP_PLayer/BP_ThirdPersonCharacterKYB.Peixes` 15.0 _returnvalue)
        (`/Game/KillYourBabiesBPS/Peixes/Os_3_Peixes/BP_Peixes1.PeixeUpdate` _returnvalue_2)
        (elif (and (`/Game/KillYourBabiesBPS/BP_PLayer/BP_ThirdPersonCharacterKYB.Has3PenguinReady` _returnvalue) (> _peixes 20.0))
          (set `/Game/KillYourBabiesBPS/BP_PLayer/BP_ThirdPersonCharacterKYB.Peixes` 20.0 _returnvalue)
          (`/Game/KillYourBabiesBPS/Peixes/Os_3_Peixes/BP_Peixes1.PeixeUpdate` _returnvalue_2)
          (elif (and (`/Game/KillYourBabiesBPS/BP_PLayer/BP_ThirdPersonCharacterKYB.Has4PenguinReady` _returnvalue) (> _peixes 25.0))
            (set `/Game/KillYourBabiesBPS/BP_PLayer/BP_ThirdPersonCharacterKYB.Peixes` 25.0 _returnvalue)
            (`/Game/KillYourBabiesBPS/Peixes/Os_3_Peixes/BP_Peixes1.PeixeUpdate` _returnvalue_2)))))))

(fn `UserConstructionScript`)