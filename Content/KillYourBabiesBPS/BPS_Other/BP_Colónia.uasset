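; BP_Colónia is the colony the player feeds with fish, owning the hunger meter and score HUD.
; Tick drains hunger in time-based tiers that steepen up to 360 seconds, then stop.
; Sphere overlap takes the player's fish, raising hunger by the cumulative delivered total.
; Tick also writes a time-plus-deliveries score to GameManager, and below zero hunger shows game over, stops FMOD events and pauses.
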(event `DecreaseHungerBar`
  (if (<= (`self.Tempo`) 100.0)
    (set `self.Hunger` (- (`self.Hunger`) 0.001))
    (elif (<= (`self.Tempo`) 180.0)
      (set `self.Hunger` (- (`self.Hunger`) 0.015))
      (elif (<= (`self.Tempo`) 240.0)
        (set `self.Hunger` (- (`self.Hunger`) 0.022))
        (elif (<= (`self.Tempo`) 300.0)
          (set `self.Hunger` (- (`self.Hunger`) 0.03))
          (elif (<= (`self.Tempo`) 360.0)
            (set `self.Hunger` (- (`self.Hunger`) 0.04))))))))

(event `self.ReceiveTick`
  (params (DeltaSeconds :type "Float (single-precision)"))
  (if (`self.HungerStarted`)
    (if (< (`self.Hunger`) 0.0)
      (bind _returnvalue (`|CreateWidget` "/Game/UI/GameOverScreen.GameOverScreen_C"))
      (`UserWidget.AddToViewport` _returnvalue 0)
      (bind _returnvalue_2 (`GameplayStatics.GetActorOfClass` "/Game/KillYourBabiesBPS/BPS_Foca/FocaTentativa.FocaTentativa_C"))
      (bind _returnvalue_3 (`GameplayStatics.GetActorOfClass` "/Game/KillYourBabiesBPS/TriggersAtivaçãoFome/TriggerExit.TriggerExit_C"))
      (`FMODBlueprintStatics.EventInstanceStop` (`/Game/KillYourBabiesBPS/BPS_Foca/FocaTentativa.ChaseInstance` _returnvalue_2))
      (`FMODBlueprintStatics.EventInstanceStop` (`/Game/KillYourBabiesBPS/TriggersAtivaçãoFome/TriggerExit.droneInstance` _returnvalue_3))
      (`GameplayStatics.SetGamePaused` true)
      (else
        (`self.DecreaseHungerBar`)
        (set `self.Tempo` (+ (`self.Tempo`) DeltaSeconds))
        (if (`self.ScoreStarted`)
          (bind _returnvalue_4 (`GameplayStatics.GetActorOfClass` "/Game/KillYourBabiesBPS/Penguins/BP_PenguinManager.BP_PenguinManager_C"))
          (bind _output_get (set `self.TimerScore` (+ (`self.TimerScore`) 0.01)))
          (bind _output_get_2 (set `self.Highscore` (+ _output_get (* (`self.PeixesEntregues`) (`/Game/KillYourBabiesBPS/Penguins/BP_PenguinManager.ScoreMultiplier` _returnvalue_4)))))
          (bind _asgame_manager (cast `/Game/KillYourBabiesBPS/GameInstance/GameManager` (`GameplayStatics.GetGameInstance`)))
          (set `/Game/KillYourBabiesBPS/GameInstance/GameManager.GlobalPlayerScore` (`KismetMathLibrary.FTrunc` _output_get_2) _asgame_manager))))
    (elif (`self.HungerAppeared`)
      (`Widget.SetVisibility` (stale `self.ReceiveBeginPlay` _returnvalue_2) "Visible")
      (`Widget.SetVisibility` (stale `self.ReceiveBeginPlay` _returnvalue_3) "Visible"))))

(event `self.ReceiveBeginPlay`
  (bind _returnvalue (`GameplayStatics.GetPlayerController` 0))
  (set `self.Hunger` 100.0)
  (bind _returnvalue_2 (`|CreateWidget` "/Game/UI/UI_Hunger.UI_Hunger_C" _returnvalue))
  (`UserWidget.AddToViewport` _returnvalue_2 0)
  (`Widget.SetVisibility` _returnvalue_2 "Hidden")
  (bind _returnvalue_3 (`|CreateWidget` "/Game/UI/UI_Score.UI_Score_C" _returnvalue))
  (`UserWidget.AddToViewport` _returnvalue_3 0)
  (`Widget.SetVisibility` _returnvalue_3 "Hidden"))

(event `self.Sphere.OnComponentBeginOverlap`
  (params (OverlappedComponent :type "PrimitiveComponent Object Reference") (OtherActor :type "Actor Object Reference") (OtherComp :type "PrimitiveComponent Object Reference") (OtherBodyIndex :type Integer) (bFromSweep :type Boolean) (SweepResult :type "HitResult Structure (by ref)"))
  (bind _asbp_third_person_character_kyb (cast `/Game/KillYourBabiesBPS/BP_PLayer/BP_ThirdPersonCharacterKYB` OtherActor))
  (if (> (`/Game/KillYourBabiesBPS/BP_PLayer/BP_ThirdPersonCharacterKYB.Peixes` _asbp_third_person_character_kyb) 0.0)
    (bind _returnvalue (`GameplayStatics.GetActorOfClass` "BP_Colónia_C"))
    (bind _returnvalue_2 (`GameplayStatics.GetActorOfClass` "/Game/KillYourBabiesBPS/Penguins/BP_PenguinManager.BP_PenguinManager_C"))
    (bind _peixes (`/Game/KillYourBabiesBPS/BP_PLayer/BP_ThirdPersonCharacterKYB.Peixes` _asbp_third_person_character_kyb))
    (bind _output_get (set `self.PeixesEntregues` (+ _peixes (`self.PeixesEntregues`))))
    (bind _returnvalue_3 (* (* _peixes 10.0) (`/Game/KillYourBabiesBPS/Penguins/BP_PenguinManager.ScoreMultiplier` _returnvalue_2)))
    (set `self.EntregaColónia` (+ (`self.EntregaColónia`) _returnvalue_3))
    (`KismetSystemLibrary.PrintString` (`KismetStringLibrary.Conv_DoubleToString` _returnvalue_3))
    (set `/Game/KillYourBabiesBPS/BPS_Other/BP_Colónia.Hunger` (+ (`self.Hunger`) _output_get) _returnvalue)
    (`KismetSystemLibrary.Delay` 0.1)
    (set `/Game/KillYourBabiesBPS/BP_PLayer/BP_ThirdPersonCharacterKYB.Peixes` 0.0 _asbp_third_person_character_kyb)
    (if (> (`self.Hunger`) 100.0)
      (set `self.Hunger` 100.0))))

(fn `UserConstructionScript`)