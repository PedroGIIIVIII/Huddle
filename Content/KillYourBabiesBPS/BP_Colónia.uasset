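; BP_Colónia is the colony actor that runs the hunger, score and game-over loop of a fish-delivery game.
; Once started, Hunger drains each Tick in steps that steepen every minute, stopping after about five minutes, and pauses into GameOverScreen below zero.
; Overlapping its sphere deposits the player's fish, restoring Hunger and adding to a score that also grows per frame.
; BeginPlay creates hidden hunger and score widgets, revealed by HungerAppeared.
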(event `DecreaseHungerBar`
  (if (<= (`self.Tempo`) 59.0)
    (set `self.Hunger` (- (`self.Hunger`) 0.01))
    (elif (<= (`self.Tempo`) 119.0)
      (set `self.Hunger` (- (`self.Hunger`) 0.02))
      (elif (<= (`self.Tempo`) 179.0)
        (set `self.Hunger` (- (`self.Hunger`) 0.03))
        (elif (<= (`self.Tempo`) 239.0)
          (set `self.Hunger` (- (`self.Hunger`) 0.04))
          (elif (<= (`self.Tempo`) 299.0)
            (set `self.Hunger` (- (`self.Hunger`) 0.05))))))))

(event `self.ReceiveTick`
  (params (DeltaSeconds :type "Float (single-precision)"))
  (if (`self.HungerStarted`)
    (if (< (`self.Hunger`) 0.0)
      (bind _returnvalue (`|CreateWidget` "/Game/UI/GameOverScreen.GameOverScreen_C"))
      (`UserWidget.AddToViewport` _returnvalue 0)
      (`GameplayStatics.SetGamePaused` true)
      (else
        (`self.DecreaseHungerBar`)
        (set `self.Tempo` (+ (`self.Tempo`) DeltaSeconds))
        (if (`self.ScoreStarted`)
          (bind _output_get (set `self.TimerScore` (+ (`self.TimerScore`) 0.01)))
          (set `self.Highscore` (+ _output_get (* (`self.PeixesEntregues`) 5.0))))))
    (elif (`self.HungerAppeared`)
      (`Widget.SetVisibility` (stale `self.ReceiveBeginPlay` _returnvalue_2) "Visible")
      (`Widget.SetVisibility` (stale `self.ReceiveBeginPlay` _returnvalue_3) "Visible"))))

(event `self.ReceiveBeginPlay`
  (bind _returnvalue (`GameplayStatics.GetPlayerController` 0))
  (set `self.Hunger` 100.0)
  (bind _returnvalue_2 (`|CreateWidget` "/Game/UI/UI_Hunger.UI_Hunger_C" _returnvalue))
  (`UserWidget.AddToViewport` _returnvalue_2 0)
  (`Widget.SetVisibility` _returnvalue_2 "Hidden")
  (bind _returnvalue_3 (`|CreateWidget` "/Game/UI/UI_Score.UI_Score_C" _returnvalue))
  (`UserWidget.AddToViewport` _returnvalue_3 0)
  (`Widget.SetVisibility` _returnvalue_3 "Hidden"))

(event `self.Sphere.OnComponentBeginOverlap`
  (params (OverlappedComponent :type "PrimitiveComponent Object Reference") (OtherActor :type "Actor Object Reference") (OtherComp :type "PrimitiveComponent Object Reference") (OtherBodyIndex :type Integer) (bFromSweep :type Boolean) (SweepResult :type "HitResult Structure (by ref)"))
  (bind _asbp_third_person_character_kyb (cast `/Game/KillYourBabiesBPS/VersãoNormal3ªPessoa/BP_ThirdPersonCharacterKYB` OtherActor))
  (bind _returnvalue (`GameplayStatics.GetActorOfClass` "BP_Colónia_C"))
  (bind _peixes (`/Game/KillYourBabiesBPS/VersãoNormal3ªPessoa/BP_ThirdPersonCharacterKYB.Peixes` _asbp_third_person_character_kyb))
  (set `self.PeixesEntregues` (+ _peixes (`self.PeixesEntregues`)))
  (set `/Game/KillYourBabiesBPS/BP_Colónia.Hunger` (+ (`self.Hunger`) (* _peixes 5.0)) _returnvalue)
  (`KismetSystemLibrary.Delay` 0.1)
  (set `/Game/KillYourBabiesBPS/VersãoNormal3ªPessoa/BP_ThirdPersonCharacterKYB.Peixes` 0.0 _asbp_third_person_character_kyb))

(fn `UserConstructionScript`)