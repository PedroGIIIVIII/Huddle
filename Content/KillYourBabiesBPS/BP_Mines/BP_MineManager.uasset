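; BP_MineManager populates the level with mines at BP_MineSpawnPoint locations when play begins.
; It gathers and shuffles all spawn points, then calls SpawnMineAtFreePoint twenty times.
; Each call picks a random point absent from ActiveMineMap, spawns a BP_Mine with that point's location and rotation, and records the pair in the map.
; The mine also receives a reference to its spawn point.
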(event `self.ReceiveBeginPlay`
  (bind _outactors (`GameplayStatics.GetAllActorsOfClass` "/Game/KillYourBabiesBPS/BP_Mines/BP_MineSpawnPoint.BP_MineSpawnPoint_C"))
  (bind _output_get (set `self.MinePointsArray` _outactors))
  (`KismetArrayLibrary.Array_Shuffle` _output_get)
  (for _ (range 20)
    (`self.SpawnMineAtFreePoint`)))

(fn `SpawnMineAtFreePoint`
  (locals (FreeMinePoints :type "Array of /Game/KillYourBabiesBPS/BP_Mines/BP_MineSpawnPoint Object Reference"))
  (bind _freeminepoints (`local.FreeMinePoints`))
  (bind _returnvalue (`KismetArrayLibrary.Array_Length` _freeminepoints))
  (for _array_element (`self.MinePointsArray`)
    (if (not (`BlueprintMapLibrary.Map_Contains` (`self.ActiveMineMap`) _array_element))
      (`KismetArrayLibrary.Array_Add` _freeminepoints _array_element)))
  (if (> _returnvalue 0)
    (bind _output_get (set `self.SelectedMineSpawnPoint` (`|GetArrayItem` _freeminepoints (`KismetMathLibrary.RandomIntegerInRange` 0 (+ _returnvalue -1)))))
    (bind _returnvalue_2 (`|SpawnActorFromClass` "/Game/KillYourBabiesBPS/BP_Mines/BP_Mine.BP_Mine_C" (`KismetMathLibrary.MakeTransform` (`self.K2_GetActorLocation` _output_get) (`self.K2_GetActorRotation` _output_get)) "Undefined" "MultiplyWithRoot" null null))
    (set `/Game/KillYourBabiesBPS/BP_Mines/BP_Mine.ThisMineSpawnPoint` _output_get _returnvalue_2)
    (`BlueprintMapLibrary.Map_Add` (`self.ActiveMineMap`) _output_get _returnvalue_2)))

(fn `UserConstructionScript`)