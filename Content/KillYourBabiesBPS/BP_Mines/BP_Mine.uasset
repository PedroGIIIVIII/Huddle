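; Floating sea mine that costs the player a visible penguin on contact, or triggers game over when none remain (tutorial hint instead if TutorialManager exists).
; DefineNaturalMoveParams starts a randomised sine bob; MoveAwayDinâmico uses retried sphere traces and player-distance checks to pick random relocation targets, re-fired from Tick.
; Detonation plays effects, updates BP_Peixes1, has BP_MineManager spawn another mine, then destroys itself, clearing its map entry.
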(event `StartIdleFloat`
  (bind (_direction _newtrack_0) (`Timeline|Timeline` :!via `PlayFromStart`)
    (:`Update`
      (`SceneComponent.K2_SetRelativeLocation` (`self.DefaultSceneRoot`) (+ (`KismetMathLibrary.MakeVector` (* (`KismetMathLibrary.Sin` (+ (* _newtrack_0 (`self.SpeedX_0`)) (`self.RandomSeedx_0`))) (`self.AmplitudeX_0`)) (* (`KismetMathLibrary.Sin` (+ (* _newtrack_0 (`self.SpeedY_0`)) (`self.RandomSeedy_0`))) (`self.AmplitudeY_0`)) (* (`KismetMathLibrary.Sin` (+ (* _newtrack_0 (`self.SpeedZ_0`)) (`self.RandomSeedz_0`))) (`self.AmplitudeZ_0`))) (`self.OriginalLocation_0`)) false false))))

(event `DefineNaturalMoveParams`
  (set `self.OriginalLocation_0` (`SceneComponent.RelativeLocation` (`self.DefaultSceneRoot`)))
  (set `self.RandomSeedx_0` (`KismetMathLibrary.RandomFloatInRange` 0.0 1000.0))
  (set `self.RandomSeedy_0` (`KismetMathLibrary.RandomFloatInRange` 0.0 1000.0))
  (set `self.RandomSeedz_0` (`KismetMathLibrary.RandomFloatInRange` 0.0 1000.0))
  (set `self.SpeedX_0` 1.0)
  (set `self.SpeedY_0` 1.0)
  (set `self.SpeedZ_0` 1.0)
  (set `self.AmplitudeX_0` (`KismetMathLibrary.RandomFloatInRange` 150.0 200.0))
  (set `self.AmplitudeY_0` (`KismetMathLibrary.RandomFloatInRange` 150.0 200.0))
  (set `self.AmplitudeZ_0` (`KismetMathLibrary.RandomFloatInRange` 150.0 200.0))
  (`self.StartIdleFloat`))

(event `self.ReceiveBeginPlay`
  (`KismetSystemLibrary.Delay` (`KismetMathLibrary.RandomFloatInRange` 1.0 5.0))
  (`FMODAudioComponent.Play` (`self.FMODAudioBipBip`)))

(event `MoveAwayDinâmico`
  (bind _targetlocation (`self.TargetLocation`))
  (set `self.CanMoveAgain` false)
  (bind _output_get (set `self.StartLocation` (`SceneComponent.K2_GetComponentLocation` (`self.DefaultSceneRoot`)) :!label _label))
  (bind _output_get_2 (set `self.TargetLocation` (+ (* (`KismetMathLibrary.RandomUnitVector`) (`KismetMathLibrary.RandomFloatInRange` 300.0 350.0)) (`self.StartLocation`))))
  (bind (_outhit _returnvalue) (`KismetSystemLibrary.SphereTraceSingle` :`Start` _output_get :`End` _output_get_2 :`Radius` 50.0 :`TraceChannel` "TraceTypeQuery1" :`bTraceComplex` true :`DrawDebugType` "ForDuration" :`DrawTime` 3.0))
  (if _returnvalue
    (bind _counter (`/Engine/EditorBlueprintResources/StandardMacros.Do N` 15 :!label _label_2)
      (:`Exit`
        (if (>= _counter 15)
          _
          (else
            (goto _label))))))
  (bind _returnvalue_2 (`GameplayStatics.GetActorOfClass` "/Game/KillYourBabiesBPS/BP_PLayer/BP_ThirdPersonCharacterKYB.BP_ThirdPersonCharacterKYB_C"))
  (if (<= (`KismetMathLibrary.Vector_Distance` (`self.TargetLocation`) (`SceneComponent.K2_GetComponentLocation` (`Character.CapsuleComponent` _returnvalue_2))) 1000.0)
    (bind _counter_2 (`/Engine/EditorBlueprintResources/StandardMacros.Do N` 15 :!label _label_3)
      (:`Exit`
        (if (>= _counter_2 15)
          (`KismetSystemLibrary.PrintString` "GIVE UP!")
          (bind (_direction _newtrack_2) (`Timeline|Timeline_0` :!via `PlayFromStart` :!label _label_4)
            (:`Update`
              (`self.K2_SetActorLocation` (`KismetMathLibrary.VLerp` (`self.StartLocation`) _targetlocation _newtrack_2))
              (goto _label_2 :!via `Reset`))
            (:`Finished`
              (set `self.StartLocation` _targetlocation)
              (set `self.CanMoveAgain` true)
              (goto _label_3 :!via `Reset`)))
          (else
            (goto _label)))))
    (else
      (goto _label_4 :!via `PlayFromStart`))))

(event `self.ReceiveDestroyed`
  (bind _returnvalue (`GameplayStatics.GetActorOfClass` "/Game/KillYourBabiesBPS/BP_Mines/BP_MineManager.BP_MineManager_C"))
  (`BlueprintMapLibrary.Map_Remove` (`/Game/KillYourBabiesBPS/BP_Mines/BP_MineManager.ActiveMineMap` _returnvalue) (`self.ThisMineSpawnPoint`)))

(event `self.Sphere1.OnComponentBeginOverlap`
  (params (OverlappedComponent :type "PrimitiveComponent Object Reference") (OtherActor :type "Actor Object Reference") (OtherComp :type "PrimitiveComponent Object Reference") (OtherBodyIndex :type Integer) (bFromSweep :type Boolean) (SweepResult :type "HitResult Structure (by ref)"))
  (bind _sphere1 (`self.Sphere1`))
  (bind _asbp_third_person_character_kyb (cast `/Game/KillYourBabiesBPS/BP_PLayer/BP_ThirdPersonCharacterKYB` OtherActor))
  (bind _penguin4 (`/Game/KillYourBabiesBPS/BP_PLayer/BP_ThirdPersonCharacterKYB.Penguin4` _asbp_third_person_character_kyb))
  (if (`SceneComponent.IsVisible` _penguin4)
    (`SceneComponent.SetVisibility` _sphere1 false false)
    (`SceneComponent.SetVisibility` _penguin4 false false)
    (`FMODAudioComponent.Play` (`self.FMODAudioExplosion`) :!label _label_5)
    (`SceneComponent.SetVisibility` (`self.Sphere2`) false false)
    (`ActorComponent.Activate` (`self.P_Explosion`) false)
    (`SceneComponent.SetVisibility` (`self.Mina`) false false)
    (bind _returnvalue (`GameplayStatics.GetActorOfClass` "/Game/KillYourBabiesBPS/Peixes/Os_3_Peixes/BP_Peixes1.BP_Peixes1_C"))
    (`/Game/KillYourBabiesBPS/Peixes/Os_3_Peixes/BP_Peixes1.PeixeUpdate` _returnvalue)
    (bind _returnvalue_2 (`GameplayStatics.GetActorOfClass` "/Game/KillYourBabiesBPS/BP_Mines/BP_MineManager.BP_MineManager_C"))
    (`/Game/KillYourBabiesBPS/BP_Mines/BP_MineManager.SpawnMineAtFreePoint` _returnvalue_2)
    (`KismetSystemLibrary.Delay` 3.58)
    (`self.K2_DestroyActor` self)
    (else
      (bind _penguin3 (`/Game/KillYourBabiesBPS/BP_PLayer/BP_ThirdPersonCharacterKYB.Penguin3` _asbp_third_person_character_kyb))
      (if (`SceneComponent.IsVisible` _penguin3)
        (`SceneComponent.SetVisibility` _sphere1 false false)
        (`SceneComponent.SetVisibility` _penguin3 false false)
        (goto _label_5)
        (else
          (bind _penguin2 (`/Game/KillYourBabiesBPS/BP_PLayer/BP_ThirdPersonCharacterKYB.Penguin2` _asbp_third_person_character_kyb))
          (if (`SceneComponent.IsVisible` _penguin2)
            (`SceneComponent.SetVisibility` _sphere1 false false)
            (`SceneComponent.SetVisibility` _penguin2 false false)
            (goto _label_5)
            (else
              (bind _penguin1 (`/Game/KillYourBabiesBPS/BP_PLayer/BP_ThirdPersonCharacterKYB.Penguin1` _asbp_third_person_character_kyb))
              (if (`SceneComponent.IsVisible` _penguin1)
                (`SceneComponent.SetVisibility` _sphere1 false false)
                (`SceneComponent.SetVisibility` _penguin1 false false)
                (goto _label_5)
                (else
                  (bind _returnvalue_3 (`GameplayStatics.GetActorOfClass` "/Game/KillYourBabiesBPS/Tutorial/TutorialManager.TutorialManager_C"))
                  (`/Engine/EditorBlueprintResources/StandardMacros.IsValid` _returnvalue_3
                    (:`Is Valid`
                      (`/Game/KillYourBabiesBPS/Tutorial/TutorialManager.GetUIHint` _returnvalue_3))
                    (:`Is Not Valid`
                      (bind _foundwidgets (`WidgetBlueprintLibrary.GetAllWidgetsOfClass` "/Game/UI/UI_Stamina.UI_Stamina_C"))
                      (for _array_element _foundwidgets
                        (`Widget.RemoveFromParent` _array_element))
                      (bind _returnvalue_4 (`|CreateWidget` "/Game/UI/GameOverScreen.GameOverScreen_C"))
                      (`UserWidget.AddToViewport` _returnvalue_4 0)
                      (`SceneComponent.SetVisibility` (`/Game/KillYourBabiesBPS/BP_PLayer/BP_ThirdPersonCharacterKYB.SkeletalMesh` _asbp_third_person_character_kyb) false false)
                      (bind _returnvalue_5 (`GameplayStatics.GetActorOfClass` "/Game/KillYourBabiesBPS/BPS_Foca/FocaTentativa.FocaTentativa_C"))
                      (bind _returnvalue_6 (`GameplayStatics.GetActorOfClass` "/Game/KillYourBabiesBPS/TriggersAtivaçãoFome/TriggerExit.TriggerExit_C"))
                      (`FMODBlueprintStatics.EventInstanceStop` (`/Game/KillYourBabiesBPS/BPS_Foca/FocaTentativa.ChaseInstance` _returnvalue_5) true)
                      (`FMODBlueprintStatics.EventInstanceStop` (`/Game/KillYourBabiesBPS/TriggersAtivaçãoFome/TriggerExit.droneInstance` _returnvalue_6) true)
                      (bind _returnvalue_7 (`GameplayStatics.GetActorOfClass` "/Game/Sound/SomFundo.SomFundo_C"))
                      (`AudioComponent.Stop` (`/Game/Sound/SomFundo.Chase` _returnvalue_7))
                      (`AudioComponent.Stop` (`/Game/Sound/SomFundo.Detected` _returnvalue_7))
                      (`GameplayStatics.SetGamePaused` true))))))))))))

(event `self.ReceiveTick`
  (params (DeltaSeconds :type "Float (single-precision)"))
  (if (`self.CanMoveAgain`)
    (`self.MoveAwayDinâmico`)))

(fn `UserConstructionScript`)