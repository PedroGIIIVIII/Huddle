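; BP_Peixes is a fish pickup that the third-person character eats by overlapping its sphere, up to a carry limit.
; On overlap, PeixeUpdate sets the limit from the character's penguin-ready flags, then ComerPeixe increments the fish count and destroys the actor if below it.
; On destruction, it frees its spawn point in PeixeManager and requests a new fish.
; A separate CustomEvent, not called here, does similar limit checks using penguin visibility.
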(event `CustomEvent`
  (bind _returnvalue (`GameplayStatics.GetActorOfClass` "/Game/KillYourBabiesBPS/VersãoNormal3ªPessoa/BP_ThirdPersonCharacterKYB.BP_ThirdPersonCharacterKYB_C"))
  (bind _returnvalue_2 (`SceneComponent.IsVisible` (`/Game/KillYourBabiesBPS/VersãoNormal3ªPessoa/BP_ThirdPersonCharacterKYB.Penguin2` _returnvalue)))
  (bind _returnvalue_3 (not _returnvalue_2))
  (bind _returnvalue_4 (`SceneComponent.IsVisible` (`/Game/KillYourBabiesBPS/VersãoNormal3ªPessoa/BP_ThirdPersonCharacterKYB.Penguin1` _returnvalue)))
  (if (and _returnvalue_3 (not _returnvalue_4))
    (set `self.Have0Penguins` true)
    (set `self.Have1Penguins` false)
    (set `self.Have2Penguins` false)
    (bind _peixes (`/Game/KillYourBabiesBPS/VersãoNormal3ªPessoa/BP_ThirdPersonCharacterKYB.Peixes` _returnvalue))
    (if (not (>= _peixes 2.0))
      (`ActorComponent.K2_DestroyComponent` (`self.Sphere`) :!label _label)
      (`ActorComponent.K2_DestroyComponent` (`self.Peixe`))
      (`KismetSystemLibrary.PrintString` "eaten"))
    (elif (or (and _returnvalue_2 (not _returnvalue_4)) (and _returnvalue_4 _returnvalue_3))
      (set `self.Have1Penguins` true)
      (set `self.Have0Penguins` false)
      (set `self.Have2Penguins` false)
      (if (not (>= _peixes 4.0))
        (goto _label))
      (elif (and _returnvalue_2 _returnvalue_4)
        (set `self.Have1Penguins` false)
        (set `self.Have0Penguins` false)
        (set `self.Have2Penguins` true)
        (if (not (>= _peixes 6.0))
          (goto _label))))))

(event `self.Sphere.OnComponentBeginOverlap`
  (params (OverlappedComponent :type "PrimitiveComponent Object Reference") (OtherActor :type "Actor Object Reference") (OtherComp :type "PrimitiveComponent Object Reference") (OtherBodyIndex :type Integer) (bFromSweep :type Boolean) (SweepResult :type "HitResult Structure (by ref)"))
  (cast `/Game/KillYourBabiesBPS/VersãoNormal3ªPessoa/BP_ThirdPersonCharacterKYB` OtherActor)
  (`self.PeixeUpdate`)
  (`self.ComerPeixe`)
  (`KismetSystemLibrary.PrintString` "Merge"))

(event `self.ReceiveDestroyed`
  (bind _returnvalue (`GameplayStatics.GetActorOfClass` "/Game/KillYourBabiesBPS/Peixes/PeixeManager.PeixeManager_C"))
  (`BlueprintMapLibrary.Map_Remove` (`/Game/KillYourBabiesBPS/Peixes/PeixeManager.ActiveFishMap` _returnvalue) (`self.MySpawnPoint`))
  (`/Game/KillYourBabiesBPS/Peixes/PeixeManager.SpawnFishAtPoint` _returnvalue)
  (`KismetSystemLibrary.PrintString` "Spawning?"))

(event `ComerPeixe`
  (bind _returnvalue (`GameplayStatics.GetActorOfClass` "/Game/KillYourBabiesBPS/VersãoNormal3ªPessoa/BP_ThirdPersonCharacterKYB.BP_ThirdPersonCharacterKYB_C"))
  (if (< (`/Game/KillYourBabiesBPS/VersãoNormal3ªPessoa/BP_ThirdPersonCharacterKYB.Peixes` _returnvalue) (`self.MaxPeixe`))
    (set `/Game/KillYourBabiesBPS/VersãoNormal3ªPessoa/BP_ThirdPersonCharacterKYB.Peixes` (+ (`/Game/KillYourBabiesBPS/VersãoNormal3ªPessoa/BP_ThirdPersonCharacterKYB.Peixes` _returnvalue) 1.0) _returnvalue)
    (`ActorComponent.K2_DestroyComponent` (`self.Sphere`))
    (`ActorComponent.K2_DestroyComponent` (`self.Peixe`))
    (`ActorComponent.K2_DestroyComponent` (`self.DefaultSceneRoot`))
    (`self.K2_DestroyActor` self)
    (`KismetSystemLibrary.PrintString` "eaten")))

(event `PeixeUpdate`
  (bind _returnvalue (`GameplayStatics.GetActorOfClass` "/Game/KillYourBabiesBPS/VersãoNormal3ªPessoa/BP_ThirdPersonCharacterKYB.BP_ThirdPersonCharacterKYB_C"))
  (if (`/Game/KillYourBabiesBPS/VersãoNormal3ªPessoa/BP_ThirdPersonCharacterKYB.Has0PenguinReady` _returnvalue)
    (set `self.MaxPeixe` 2.0)
    (elif (`/Game/KillYourBabiesBPS/VersãoNormal3ªPessoa/BP_ThirdPersonCharacterKYB.Has1PenguinReady` _returnvalue)
      (set `self.MaxPeixe` 4.0)
      (elif (`/Game/KillYourBabiesBPS/VersãoNormal3ªPessoa/BP_ThirdPersonCharacterKYB.Has2PenguinReady` _returnvalue)
        (set `self.MaxPeixe` 6.0)
        (elif (`/Game/KillYourBabiesBPS/VersãoNormal3ªPessoa/BP_ThirdPersonCharacterKYB.Has3PenguinReady` _returnvalue)
          (set `self.MaxPeixe` 8.0)
          (elif (`/Game/KillYourBabiesBPS/VersãoNormal3ªPessoa/BP_ThirdPersonCharacterKYB.Has4PenguinReady` _returnvalue)
            (set `self.MaxPeixe` 10.0)))))))

(fn `UserConstructionScript`)