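; Fish pickup that BP_ThirdPersonCharacterKYB eats on sphere overlap to raise its Peixes count, up to a cap.
; On overlap, PeixeUpdate reads the character's penguin-ready flags to set the cap, then nudges camera arm length and penguin formation offsets one Lerp step.
; Eating asks PeixeManager to spawn another fish, then destroys this one.
; Destruction plays a collect sound and removes its spawn point from the manager's active map.
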(event `self.Sphere.OnComponentBeginOverlap`
  (params (OverlappedComponent :type "PrimitiveComponent Object Reference") (OtherActor :type "Actor Object Reference") (OtherComp :type "PrimitiveComponent Object Reference") (OtherBodyIndex :type Integer) (bFromSweep :type Boolean) (SweepResult :type "HitResult Structure (by ref)"))
  (cast `/Game/KillYourBabiesBPS/BP_PLayer/BP_ThirdPersonCharacterKYB` OtherActor)
  (`self.PeixeUpdate`)
  (`self.ComerPeixe`)
  (`KismetSystemLibrary.PrintString` "Merge"))

(event `self.ReceiveDestroyed`
  (`FMODBlueprintStatics.PlayEvent2D` "/Game/FMOD/Events/SFX/Collect_Fish.Collect_Fish")
  (bind _returnvalue (`GameplayStatics.GetActorOfClass` "/Game/KillYourBabiesBPS/Peixes/PeixeManager.PeixeManager_C"))
  (`BlueprintMapLibrary.Map_Remove` (`/Game/KillYourBabiesBPS/Peixes/PeixeManager.ActiveFishMap` _returnvalue) (`self.MySpawnPoint`)))

(event `ComerPeixe`
  (bind _returnvalue (`GameplayStatics.GetActorOfClass` "/Game/KillYourBabiesBPS/BP_PLayer/BP_ThirdPersonCharacterKYB.BP_ThirdPersonCharacterKYB_C"))
  (if (< (`/Game/KillYourBabiesBPS/BP_PLayer/BP_ThirdPersonCharacterKYB.Peixes` _returnvalue) (`self.MaxPeixe`))
    (set `/Game/KillYourBabiesBPS/BP_PLayer/BP_ThirdPersonCharacterKYB.Peixes` (+ (`/Game/KillYourBabiesBPS/BP_PLayer/BP_ThirdPersonCharacterKYB.Peixes` _returnvalue) 1.0) _returnvalue)
    (bind _returnvalue_2 (`GameplayStatics.GetActorOfClass` "/Game/KillYourBabiesBPS/Peixes/PeixeManager.PeixeManager_C"))
    (`/Game/KillYourBabiesBPS/Peixes/PeixeManager.SpawnFishAtPoint` _returnvalue_2)
    (`self.K2_DestroyActor` self)
    (`KismetSystemLibrary.PrintString` "eaten")))

(event `PeixeUpdate`
  (bind _returnvalue (`GameplayStatics.GetActorOfClass` "/Game/KillYourBabiesBPS/BP_PLayer/BP_ThirdPersonCharacterKYB.BP_ThirdPersonCharacterKYB_C"))
  (if (`/Game/KillYourBabiesBPS/BP_PLayer/BP_ThirdPersonCharacterKYB.Has0PenguinReady` _returnvalue)
    (set `self.MaxPeixe` 2.0)
    (bind _returnvalue_2 (`GameplayStatics.GetActorOfClass` "/Game/KillYourBabiesBPS/BP_PLayer/BP_ThirdPersonCharacterKYB.BP_ThirdPersonCharacterKYB_C"))
    (bind _cameraboom (`HuddleCharacter.CameraBoom` _returnvalue_2))
    (set `SpringArmComponent.TargetArmLength` (`KismetMathLibrary.Lerp` (`SpringArmComponent.TargetArmLength` _cameraboom) 650.0 0.02) _cameraboom)
    (`self.PenguinPositions0`)
    (elif (`/Game/KillYourBabiesBPS/BP_PLayer/BP_ThirdPersonCharacterKYB.Has1PenguinReady` _returnvalue)
      (set `self.MaxPeixe` 4.0)
      (bind _returnvalue_3 (`GameplayStatics.GetActorOfClass` "/Game/KillYourBabiesBPS/BP_PLayer/BP_ThirdPersonCharacterKYB.BP_ThirdPersonCharacterKYB_C"))
      (bind _cameraboom_2 (`HuddleCharacter.CameraBoom` _returnvalue_3))
      (set `SpringArmComponent.TargetArmLength` (`KismetMathLibrary.Lerp` (`SpringArmComponent.TargetArmLength` _cameraboom_2) 700.0 0.02) _cameraboom_2)
      (`self.PenguinPositions1`)
      (elif (`/Game/KillYourBabiesBPS/BP_PLayer/BP_ThirdPersonCharacterKYB.Has2PenguinReady` _returnvalue)
        (set `self.MaxPeixe` 6.0)
        (bind _returnvalue_4 (`GameplayStatics.GetActorOfClass` "/Game/KillYourBabiesBPS/BP_PLayer/BP_ThirdPersonCharacterKYB.BP_ThirdPersonCharacterKYB_C"))
        (bind _cameraboom_3 (`HuddleCharacter.CameraBoom` _returnvalue_4))
        (set `SpringArmComponent.TargetArmLength` (`KismetMathLibrary.Lerp` (`SpringArmComponent.TargetArmLength` _cameraboom_3) 800.0 0.02) _cameraboom_3)
        (`self.PenguinPositions2`)
        (elif (`/Game/KillYourBabiesBPS/BP_PLayer/BP_ThirdPersonCharacterKYB.Has3PenguinReady` _returnvalue)
          (set `self.MaxPeixe` 8.0)
          (bind _returnvalue_5 (`GameplayStatics.GetActorOfClass` "/Game/KillYourBabiesBPS/BP_PLayer/BP_ThirdPersonCharacterKYB.BP_ThirdPersonCharacterKYB_C"))
          (bind _cameraboom_4 (`HuddleCharacter.CameraBoom` _returnvalue_5))
          (set `SpringArmComponent.TargetArmLength` (`KismetMathLibrary.Lerp` (`SpringArmComponent.TargetArmLength` _cameraboom_4) 900.0 0.02) _cameraboom_4)
          (`self.PenguinPositions3`)
          (elif (`/Game/KillYourBabiesBPS/BP_PLayer/BP_ThirdPersonCharacterKYB.Has4PenguinReady` _returnvalue)
            (set `self.MaxPeixe` 10.0)
            (bind _returnvalue_6 (`GameplayStatics.GetActorOfClass` "/Game/KillYourBabiesBPS/BP_PLayer/BP_ThirdPersonCharacterKYB.BP_ThirdPersonCharacterKYB_C"))
            (bind _cameraboom_5 (`HuddleCharacter.CameraBoom` _returnvalue_6))
            (set `SpringArmComponent.TargetArmLength` (`KismetMathLibrary.Lerp` (`SpringArmComponent.TargetArmLength` _cameraboom_5) 1000.0 0.02) _cameraboom_5)
            (`self.PenguinPositions4`)))))))

(fn `PenguinPositions0`
  (bind _returnvalue (`GameplayStatics.GetActorOfClass` "/Game/KillYourBabiesBPS/BP_PLayer/BP_ThirdPersonCharacterKYB.BP_ThirdPersonCharacterKYB_C"))
  (bind _skeletalmesh (`/Game/KillYourBabiesBPS/BP_PLayer/BP_ThirdPersonCharacterKYB.SkeletalMesh` _returnvalue))
  (bind _output_get (set `/Game/KillYourBabiesBPS/BP_PLayer/BP_ThirdPersonCharacterKYB.OriginalLocation_0` (`KismetMathLibrary.VLerp` (`SceneComponent.RelativeLocation` _skeletalmesh) (74.378734 48.315798 -164.002911) (`self.AdjustingSpeed`)) _returnvalue))
  (set `/Game/KillYourBabiesBPS/BP_PLayer/BP_ThirdPersonCharacterKYB.AmplitudeX_0` 1.0 _returnvalue)
  (set `/Game/KillYourBabiesBPS/BP_PLayer/BP_ThirdPersonCharacterKYB.AmplitudeY_0` 1.0 _returnvalue)
  (set `/Game/KillYourBabiesBPS/BP_PLayer/BP_ThirdPersonCharacterKYB.AmplitudeZ_0` 1.0 _returnvalue)
  (`SceneComponent.K2_SetRelativeLocation` _skeletalmesh _output_get false false))

(fn `PenguinPositions1`
  (bind _returnvalue (`GameplayStatics.GetActorOfClass` "/Game/KillYourBabiesBPS/BP_PLayer/BP_ThirdPersonCharacterKYB.BP_ThirdPersonCharacterKYB_C"))
  (bind _skeletalmesh (`/Game/KillYourBabiesBPS/BP_PLayer/BP_ThirdPersonCharacterKYB.SkeletalMesh` _returnvalue))
  (bind _output_get (set `/Game/KillYourBabiesBPS/BP_PLayer/BP_ThirdPersonCharacterKYB.OriginalLocation_0` (`KismetMathLibrary.VLerp` (`SceneComponent.RelativeLocation` _skeletalmesh) (-23.72205 -113.605215 -164.002913) (`self.AdjustingSpeed`)) _returnvalue))
  (set `/Game/KillYourBabiesBPS/BP_PLayer/BP_ThirdPersonCharacterKYB.AmplitudeX_0` 1.0 _returnvalue)
  (set `/Game/KillYourBabiesBPS/BP_PLayer/BP_ThirdPersonCharacterKYB.AmplitudeY_0` 1.0 _returnvalue)
  (set `/Game/KillYourBabiesBPS/BP_PLayer/BP_ThirdPersonCharacterKYB.AmplitudeZ_0` 1.0 _returnvalue)
  (`SceneComponent.K2_SetRelativeLocation` _skeletalmesh _output_get false false)
  (bind _returnvalue_2 (`GameplayStatics.GetActorOfClass` "/Game/KillYourBabiesBPS/Penguins/NaturalMovementManager.NaturalMovementManager_C"))
  (bind _penguin1 (`/Game/KillYourBabiesBPS/BP_PLayer/BP_ThirdPersonCharacterKYB.Penguin1` _returnvalue))
  (bind _output_get_2 (set `/Game/KillYourBabiesBPS/Penguins/NaturalMovementManager.OriginalLocation_1` (`KismetMathLibrary.VLerp` (`SceneComponent.RelativeLocation` _penguin1) (-10.659666 162.889961 -47.198271) (`self.AdjustingSpeed`)) _returnvalue_2))
  (set `/Game/KillYourBabiesBPS/Penguins/NaturalMovementManager.AmplitudeX_1` 1.0 _returnvalue_2)
  (set `/Game/KillYourBabiesBPS/Penguins/NaturalMovementManager.AmplitudeY_1` 1.0 _returnvalue_2)
  (set `/Game/KillYourBabiesBPS/Penguins/NaturalMovementManager.AmplitudeZ_1` 1.0 _returnvalue_2)
  (`SceneComponent.K2_SetRelativeLocation` _penguin1 _output_get_2 false false))

(fn `PenguinPositions2`
  (bind _returnvalue (`GameplayStatics.GetActorOfClass` "/Game/KillYourBabiesBPS/BP_PLayer/BP_ThirdPersonCharacterKYB.BP_ThirdPersonCharacterKYB_C"))
  (bind _skeletalmesh (`/Game/KillYourBabiesBPS/BP_PLayer/BP_ThirdPersonCharacterKYB.SkeletalMesh` _returnvalue))
  (bind _output_get (set `/Game/KillYourBabiesBPS/BP_PLayer/BP_ThirdPersonCharacterKYB.OriginalLocation_0` (`KismetMathLibrary.VLerp` (`SceneComponent.RelativeLocation` _skeletalmesh) (-23.72205 -113.605215 -174.002913) (`self.AdjustingSpeed`)) _returnvalue))
  (set `/Game/KillYourBabiesBPS/BP_PLayer/BP_ThirdPersonCharacterKYB.AmplitudeX_0` 1.0 _returnvalue)
  (set `/Game/KillYourBabiesBPS/BP_PLayer/BP_ThirdPersonCharacterKYB.AmplitudeY_0` 1.0 _returnvalue)
  (set `/Game/KillYourBabiesBPS/BP_PLayer/BP_ThirdPersonCharacterKYB.AmplitudeZ_0` 1.0 _returnvalue)
  (`SceneComponent.K2_SetRelativeLocation` _skeletalmesh _output_get false false)
  (bind _returnvalue_2 (`GameplayStatics.GetActorOfClass` "/Game/KillYourBabiesBPS/Penguins/NaturalMovementManager.NaturalMovementManager_C"))
  (bind _penguin1 (`/Game/KillYourBabiesBPS/BP_PLayer/BP_ThirdPersonCharacterKYB.Penguin1` _returnvalue))
  (bind _output_get_2 (set `/Game/KillYourBabiesBPS/Penguins/NaturalMovementManager.OriginalLocation_1` (`KismetMathLibrary.VLerp` (`SceneComponent.RelativeLocation` _penguin1) (-111.757224 39.318341 -87.365358) (`self.AdjustingSpeed`)) _returnvalue_2))
  (set `/Game/KillYourBabiesBPS/Penguins/NaturalMovementManager.AmplitudeX_1` 1.0 _returnvalue_2)
  (set `/Game/KillYourBabiesBPS/Penguins/NaturalMovementManager.AmplitudeY_1` 1.0 _returnvalue_2)
  (set `/Game/KillYourBabiesBPS/Penguins/NaturalMovementManager.AmplitudeZ_1` 1.0 _returnvalue_2)
  (`SceneComponent.K2_SetRelativeLocation` _penguin1 _output_get_2 false false)
  (bind _returnvalue_3 (`GameplayStatics.GetActorOfClass` "/Game/KillYourBabiesBPS/Penguins/NaturalMovementManager.NaturalMovementManager_C"))
  (bind _penguin2 (`/Game/KillYourBabiesBPS/BP_PLayer/BP_ThirdPersonCharacterKYB.Penguin2` _returnvalue))
  (bind _output_get_3 (set `/Game/KillYourBabiesBPS/Penguins/NaturalMovementManager.OriginalLocation_2` (`KismetMathLibrary.VLerp` (`SceneComponent.RelativeLocation` _penguin2) (-10.659666 162.889961 -47.198271) (`self.AdjustingSpeed`)) _returnvalue_3))
  (set `/Game/KillYourBabiesBPS/Penguins/NaturalMovementManager.AmplitudeX_2` 1.0 _returnvalue_3)
  (set `/Game/KillYourBabiesBPS/Penguins/NaturalMovementManager.AmplitudeY_2` 1.0 _returnvalue_3)
  (set `/Game/KillYourBabiesBPS/Penguins/NaturalMovementManager.AmplitudeZ_2` 1.0 _returnvalue_3)
  (`SceneComponent.K2_SetRelativeLocation` _penguin2 _output_get_3 false false))

(fn `PenguinPositions3`
  (bind _returnvalue (`GameplayStatics.GetActorOfClass` "/Game/KillYourBabiesBPS/BP_PLayer/BP_ThirdPersonCharacterKYB.BP_ThirdPersonCharacterKYB_C"))
  (bind _skeletalmesh (`/Game/KillYourBabiesBPS/BP_PLayer/BP_ThirdPersonCharacterKYB.SkeletalMesh` _returnvalue))
  (bind _output_get (set `/Game/KillYourBabiesBPS/BP_PLayer/BP_ThirdPersonCharacterKYB.OriginalLocation_0` (`KismetMathLibrary.VLerp` (`SceneComponent.RelativeLocation` _skeletalmesh) (3.86 -104.54 -180.0) (`self.AdjustingSpeed`)) _returnvalue))
  (set `/Game/KillYourBabiesBPS/BP_PLayer/BP_ThirdPersonCharacterKYB.AmplitudeX_0` 1.0 _returnvalue)
  (set `/Game/KillYourBabiesBPS/BP_PLayer/BP_ThirdPersonCharacterKYB.AmplitudeY_0` 1.0 _returnvalue)
  (set `/Game/KillYourBabiesBPS/BP_PLayer/BP_ThirdPersonCharacterKYB.AmplitudeZ_0` 1.0 _returnvalue)
  (`SceneComponent.K2_SetRelativeLocation` _skeletalmesh _output_get false false)
  (bind _returnvalue_2 (`GameplayStatics.GetActorOfClass` "/Game/KillYourBabiesBPS/Penguins/NaturalMovementManager.NaturalMovementManager_C"))
  (bind _penguin1 (`/Game/KillYourBabiesBPS/BP_PLayer/BP_ThirdPersonCharacterKYB.Penguin1` _returnvalue))
  (bind _output_get_2 (set `/Game/KillYourBabiesBPS/Penguins/NaturalMovementManager.OriginalLocation_1` (`KismetMathLibrary.VLerp` (`SceneComponent.RelativeLocation` _penguin1) (17.8 176.5 -96.3) (`self.AdjustingSpeed`)) _returnvalue_2))
  (set `/Game/KillYourBabiesBPS/Penguins/NaturalMovementManager.AmplitudeX_1` 1.0 _returnvalue_2)
  (set `/Game/KillYourBabiesBPS/Penguins/NaturalMovementManager.AmplitudeY_1` 1.0 _returnvalue_2)
  (set `/Game/KillYourBabiesBPS/Penguins/NaturalMovementManager.AmplitudeZ_1` 1.0 _returnvalue_2)
  (`SceneComponent.K2_SetRelativeLocation` _penguin1 _output_get_2 false false)
  (bind _returnvalue_3 (`GameplayStatics.GetActorOfClass` "/Game/KillYourBabiesBPS/Penguins/NaturalMovementManager.NaturalMovementManager_C"))
  (bind _penguin2 (`/Game/KillYourBabiesBPS/BP_PLayer/BP_ThirdPersonCharacterKYB.Penguin2` _returnvalue))
  (bind _output_get_3 (set `/Game/KillYourBabiesBPS/Penguins/NaturalMovementManager.OriginalLocation_2` (`KismetMathLibrary.VLerp` (`SceneComponent.RelativeLocation` _penguin2) (-117.2 38.5 -82.5) (`self.AdjustingSpeed`)) _returnvalue_3))
  (set `/Game/KillYourBabiesBPS/Penguins/NaturalMovementManager.AmplitudeX_2` 1.0 _returnvalue_3)
  (set `/Game/KillYourBabiesBPS/Penguins/NaturalMovementManager.AmplitudeY_2` 1.0 _returnvalue_3)
  (set `/Game/KillYourBabiesBPS/Penguins/NaturalMovementManager.AmplitudeZ_2` 1.0 _returnvalue_3)
  (`SceneComponent.K2_SetRelativeLocation` _penguin2 _output_get_3 false false)
  (bind _returnvalue_4 (`GameplayStatics.GetActorOfClass` "/Game/KillYourBabiesBPS/Penguins/NaturalMovementManager.NaturalMovementManager_C"))
  (bind _penguin3 (`/Game/KillYourBabiesBPS/BP_PLayer/BP_ThirdPersonCharacterKYB.Penguin3` _returnvalue))
  (bind _output_get_4 (set `/Game/KillYourBabiesBPS/Penguins/NaturalMovementManager.OriginalLocation_3` (`KismetMathLibrary.VLerp` (`SceneComponent.RelativeLocation` _penguin3) (140.1 28.92 -61.0) (`self.AdjustingSpeed`)) _returnvalue_4))
  (set `/Game/KillYourBabiesBPS/Penguins/NaturalMovementManager.AmplitudeX_3` 1.0 _returnvalue_4)
  (set `/Game/KillYourBabiesBPS/Penguins/NaturalMovementManager.AmplitudeY_3` 1.0 _returnvalue_4)
  (set `/Game/KillYourBabiesBPS/Penguins/NaturalMovementManager.AmplitudeZ_3` 1.0 _returnvalue_4)
  (`SceneComponent.K2_SetRelativeLocation` _penguin3 _output_get_4 false false))

(fn `PenguinPositions4`
  (bind _returnvalue (`GameplayStatics.GetActorOfClass` "/Game/KillYourBabiesBPS/BP_PLayer/BP_ThirdPersonCharacterKYB.BP_ThirdPersonCharacterKYB_C"))
  (bind _skeletalmesh (`/Game/KillYourBabiesBPS/BP_PLayer/BP_ThirdPersonCharacterKYB.SkeletalMesh` _returnvalue))
  (bind _output_get (set `/Game/KillYourBabiesBPS/BP_PLayer/BP_ThirdPersonCharacterKYB.OriginalLocation_0` (`KismetMathLibrary.VLerp` (`SceneComponent.RelativeLocation` _skeletalmesh) (19.91 -130.14 -42.132) (`self.AdjustingSpeed`)) _returnvalue))
  (set `/Game/KillYourBabiesBPS/BP_PLayer/BP_ThirdPersonCharacterKYB.AmplitudeX_0` 1.0 _returnvalue)
  (set `/Game/KillYourBabiesBPS/BP_PLayer/BP_ThirdPersonCharacterKYB.AmplitudeY_0` 1.0 _returnvalue)
  (set `/Game/KillYourBabiesBPS/BP_PLayer/BP_ThirdPersonCharacterKYB.AmplitudeZ_0` 1.0 _returnvalue)
  (`SceneComponent.K2_SetRelativeLocation` _skeletalmesh _output_get false false)
  (bind _returnvalue_2 (`GameplayStatics.GetActorOfClass` "/Game/KillYourBabiesBPS/Penguins/NaturalMovementManager.NaturalMovementManager_C"))
  (bind _penguin1 (`/Game/KillYourBabiesBPS/BP_PLayer/BP_ThirdPersonCharacterKYB.Penguin1` _returnvalue))
  (bind _output_get_2 (set `/Game/KillYourBabiesBPS/Penguins/NaturalMovementManager.OriginalLocation_1` (`KismetMathLibrary.VLerp` (`SceneComponent.RelativeLocation` _penguin1) (4.25 165.66 -94.387) (`self.AdjustingSpeed`)) _returnvalue_2))
  (set `/Game/KillYourBabiesBPS/Penguins/NaturalMovementManager.AmplitudeX_1` 1.0 _returnvalue_2)
  (set `/Game/KillYourBabiesBPS/Penguins/NaturalMovementManager.AmplitudeY_1` 1.0 _returnvalue_2)
  (set `/Game/KillYourBabiesBPS/Penguins/NaturalMovementManager.AmplitudeZ_1` 1.0 _returnvalue_2)
  (`SceneComponent.K2_SetRelativeLocation` _penguin1 _output_get_2 false false)
  (bind _returnvalue_3 (`GameplayStatics.GetActorOfClass` "/Game/KillYourBabiesBPS/Penguins/NaturalMovementManager.NaturalMovementManager_C"))
  (bind _penguin2 (`/Game/KillYourBabiesBPS/BP_PLayer/BP_ThirdPersonCharacterKYB.Penguin2` _returnvalue))
  (bind _output_get_3 (set `/Game/KillYourBabiesBPS/Penguins/NaturalMovementManager.OriginalLocation_2` (`KismetMathLibrary.VLerp` (`SceneComponent.RelativeLocation` _penguin2) (-21.71 -90.283 -95.049) (`self.AdjustingSpeed`)) _returnvalue_3))
  (set `/Game/KillYourBabiesBPS/Penguins/NaturalMovementManager.AmplitudeX_2` 1.0 _returnvalue_3)
  (set `/Game/KillYourBabiesBPS/Penguins/NaturalMovementManager.AmplitudeY_2` 1.0 _returnvalue_3)
  (set `/Game/KillYourBabiesBPS/Penguins/NaturalMovementManager.AmplitudeZ_2` 1.0 _returnvalue_3)
  (`SceneComponent.K2_SetRelativeLocation` _penguin2 _output_get_3 false false)
  (bind _returnvalue_4 (`GameplayStatics.GetActorOfClass` "/Game/KillYourBabiesBPS/Penguins/NaturalMovementManager.NaturalMovementManager_C"))
  (bind _penguin3 (`/Game/KillYourBabiesBPS/BP_PLayer/BP_ThirdPersonCharacterKYB.Penguin3` _returnvalue))
  (bind _output_get_4 (set `/Game/KillYourBabiesBPS/Penguins/NaturalMovementManager.OriginalLocation_3` (`KismetMathLibrary.VLerp` (`SceneComponent.RelativeLocation` _penguin3) (141.655 28.92 -50.007) (`self.AdjustingSpeed`)) _returnvalue_4))
  (set `/Game/KillYourBabiesBPS/Penguins/NaturalMovementManager.AmplitudeX_3` 1.0 _returnvalue_4)
  (set `/Game/KillYourBabiesBPS/Penguins/NaturalMovementManager.AmplitudeY_3` 1.0 _returnvalue_4)
  (set `/Game/KillYourBabiesBPS/Penguins/NaturalMovementManager.AmplitudeZ_3` 1.0 _returnvalue_4)
  (`SceneComponent.K2_SetRelativeLocation` _penguin3 _output_get_4 false false)
  (bind _returnvalue_5 (`GameplayStatics.GetActorOfClass` "/Game/KillYourBabiesBPS/Penguins/NaturalMovementManager.NaturalMovementManager_C"))
  (bind _penguin4 (`/Game/KillYourBabiesBPS/BP_PLayer/BP_ThirdPersonCharacterKYB.Penguin4` _returnvalue))
  (bind _output_get_5 (set `/Game/KillYourBabiesBPS/Penguins/NaturalMovementManager.OriginalLocation_4` (`KismetMathLibrary.VLerp` (`SceneComponent.RelativeLocation` _penguin4) (-39.179 190.0 55.0) (`self.AdjustingSpeed`)) _returnvalue_5))
  (set `/Game/KillYourBabiesBPS/Penguins/NaturalMovementManager.AmplitudeX_4` 1.0 _returnvalue_5)
  (set `/Game/KillYourBabiesBPS/Penguins/NaturalMovementManager.AmplitudeY_4` 1.0 _returnvalue_5)
  (set `/Game/KillYourBabiesBPS/Penguins/NaturalMovementManager.AmplitudeZ_4` 1.0 _returnvalue_5)
  (`SceneComponent.K2_SetRelativeLocation` _penguin4 _output_get_5 false false))

(fn `UserConstructionScript`)