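; Collectible fish that randomly becomes one of three types, worth increasing amounts to the player.
; Common fish dart to sphere-traced clear points, uncommon ones bob on sine waves and face nearby players, rare ones follow a spline.
; Non-spline fish turn toward the seal while it follows.
; On player overlap, penguin state sets fish capacity and nudges camera and penguin formation; below capacity, the fish is counted, destroyed and respawned through PeixeManager.
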(event `StartIdleFloat`
  (bind (_direction _newtrack_0) (`Timeline|Timeline` :!via `PlayFromStart`)
    (:`Update`
      (`SceneComponent.K2_SetRelativeLocation` (`self.DefaultSceneRoot`) (+ (`KismetMathLibrary.MakeVector` (* (`KismetMathLibrary.Sin` (+ (* _newtrack_0 (`self.SpeedX_0`)) (`self.RandomSeedx_0`))) (`self.AmplitudeX_0`)) (* (`KismetMathLibrary.Sin` (+ (* _newtrack_0 (`self.SpeedY_0`)) (`self.RandomSeedy_0`))) (`self.AmplitudeY_0`)) (* (`KismetMathLibrary.Sin` (+ (* _newtrack_0 (`self.SpeedZ_0`)) (`self.RandomSeedz_0`))) (`self.AmplitudeZ_0`))) (`self.OriginalLocation_0`)) false false))))

(event `DefineNaturalMoveParams`
  (set `self.OriginalLocation_0` (`SceneComponent.RelativeLocation` (`self.DefaultSceneRoot`)))
  (set `self.RandomSeedx_0` (`KismetMathLibrary.RandomFloatInRange` 0.0 1000.0))
  (set `self.RandomSeedy_0` (`KismetMathLibrary.RandomFloatInRange` 0.0 1000.0))
  (set `self.RandomSeedz_0` (`KismetMathLibrary.RandomFloatInRange` 0.0 1000.0))
  (set `self.SpeedX_0` 5.0)
  (set `self.SpeedY_0` 5.0)
  (set `self.SpeedZ_0` 5.0)
  (set `self.AmplitudeX_0` (`KismetMathLibrary.RandomFloatInRange` 10.0 25.0))
  (set `self.AmplitudeY_0` (`KismetMathLibrary.RandomFloatInRange` 10.0 25.0))
  (set `self.AmplitudeZ_0` (`KismetMathLibrary.RandomFloatInRange` 10.0 40.0))
  (`self.StartIdleFloat`))

(event `MoveAway`
  (bind _targetlocation (`self.TargetLocation`))
  (set `self.CanMoveAgain` false)
  (bind _output_get (set `self.StartLocation` (`SceneComponent.K2_GetComponentLocation` (`self.DefaultSceneRoot`))))
  (bind _output_get_2 (set `self.TargetLocation` (+ (* (`KismetMathLibrary.RandomUnitVector`) (`KismetMathLibrary.RandomFloatInRange` 700.0 1500.0)) (`self.StartLocation`)) :!label _label))
  (bind (_outhit _returnvalue) (`KismetSystemLibrary.SphereTraceSingle` _output_get _output_get_2 100.0 "TraceTypeQuery1"))
  (if _returnvalue
    (goto _label)
    (else
      (bind (_direction _newtrack_0) (`Timeline|Timeline_0` :!via `PlayFromStart`)
        (:`Update`
          (`self.K2_SetActorLocation` (`KismetMathLibrary.VLerp` (`self.StartLocation`) _targetlocation _newtrack_0)))
        (:`Finished`
          (set `self.StartLocation` _targetlocation)
          (bind _output_get_3 (set `self.Timeline_0` (`self.Timeline_0`)))
          (`TimelineComponent.SetTimelineLength` _output_get_3 (`KismetMathLibrary.RandomFloatInRange` 3.5 4.5))
          (set `self.CanMoveAgain` true))))))

(event `self.ReceiveBeginPlay`
  (bind _output_get (set `self.SortedFish` (`KismetMathLibrary.RandomFloatInRange` 0.0 100.0)))
  (if (<= _output_get 70.0)
    (`PrimitiveComponent.SetMaterial` (`self.Peixe`) 0 "/Game/Assets/Modelos/Models/Rigged/Peixe/Fish_Texture2.Fish_Texture2")
    (set `self.PeixeTipo1` true)
    (set `self.PeixeTipo2` false)
    (elif (<= _output_get 95.0)
      (`PrimitiveComponent.SetMaterial` (`self.Peixe`) 0 "/Game/Assets/Modelos/Models/Rigged/Peixe/Fish_Texture1.Fish_Texture1")
      (set `self.PeixeTipo1` false)
      (set `self.PeixeTipo2` true)
      (`self.DefineNaturalMoveParams`)
      (else
        (`PrimitiveComponent.SetMaterial` (`self.Peixe`) 0 "/Game/Assets/Modelos/Models/Rigged/Peixe/Fish_Texture3.Fish_Texture3")
        (set `self.PeixeTipo1` false)
        (set `self.PeixeTipo2` false)
        (bind _returnvalue (`GameplayStatics.GetActorOfClass` "/Game/KillYourBabiesBPS/Peixes/Os_3_Peixes/Peixe3/SplineFor3ºFish.SplineFor3ºFish_C"))
        (bind _output_get_2 (set `self.SplineLenght` (`SplineComponent.GetSplineLength` (`/Game/KillYourBabiesBPS/Peixes/Os_3_Peixes/Peixe3/SplineFor3ºFish.Spline1` _returnvalue))))
        (set `self.RandomSplinePoint` (`KismetMathLibrary.RandomFloatInRange` 0.0 _output_get_2))))))

(event `3ºPeixe`
  (bind _splinelenght (`self.SplineLenght`))
  (bind _randomsplinepoint (`self.RandomSplinePoint`))
  (bind _defaultsceneroot (`self.DefaultSceneRoot`))
  (bind _output_get (set `self.RandomSplinePoint` (+ (* (`self.Speed3ºFish`) (stale `self.ReceiveTick` DeltaSeconds)) (`self.RandomSplinePoint`))))
  (bind _returnvalue (`SplineComponent.GetTransformAtDistanceAlongSpline` (`/Game/KillYourBabiesBPS/Peixes/Os_3_Peixes/Peixe3/SplineFor3ºFish.Spline1` (stale `self.ReceiveBeginPlay` _returnvalue)) _output_get "World" false))
  (`SceneComponent.K2_SetRelativeTransform` _defaultsceneroot (`KismetMathLibrary.MakeTransform` (`KismetMathLibrary.MakeVector` (.x (.location _returnvalue)) (.y (.location _returnvalue)) (.z (.location _returnvalue))) (`KismetMathLibrary.RInterpTo` (`SceneComponent.K2_GetComponentRotation` _defaultsceneroot) (`KismetMathLibrary.MakeRotator` (.roll (.rotation _returnvalue)) (.pitch (.rotation _returnvalue)) (.yaw (.rotation _returnvalue))) (stale `self.ReceiveTick` DeltaSeconds) 3.0) (5.0 5.0 5.0)) false false)
  (if (`self.Loop`)
    (`KismetSystemLibrary.PrintString` (`KismetStringLibrary.Conv_DoubleToString` _randomsplinepoint))
    (`KismetSystemLibrary.PrintString` (`KismetStringLibrary.Conv_DoubleToString` _splinelenght))
    (if (> _randomsplinepoint _splinelenght)
      (set `self.RandomSplinePoint` 0.0))))

(event `self.Sphere.OnComponentBeginOverlap`
  (params (OverlappedComponent :type "PrimitiveComponent Object Reference") (OtherActor :type "Actor Object Reference") (OtherComp :type "PrimitiveComponent Object Reference") (OtherBodyIndex :type Integer) (bFromSweep :type Boolean) (SweepResult :type "HitResult Structure (by ref)"))
  (cast `/Game/KillYourBabiesBPS/BP_PLayer/BP_ThirdPersonCharacterKYB` OtherActor)
  (`self.PeixeUpdate`)
  (`self.ComerPeixe`)
  (`KismetSystemLibrary.PrintString` "Merge"))

(event `self.ReceiveTick`
  (params (DeltaSeconds :type "Float (single-precision)"))
  (bind _peixe (`self.Peixe`))
  (bind _peixe_2 (`self.Peixe`))
  (bind _defaultsceneroot (`self.DefaultSceneRoot`))
  (bind _targetlocation (`self.TargetLocation`))
  (bind _returnvalue (`SceneComponent.K2_GetComponentLocation` _peixe_2))
  (bind _returnvalue_2 (`SceneComponent.K2_GetComponentRotation` _peixe_2))
  (bind (_returnvalue_roll _returnvalue_pitch _returnvalue_yaw) (`KismetMathLibrary.BreakRotator` (`KismetMathLibrary.FindLookAtRotation` _returnvalue (+ (`self.TargetLocation`) (* (`KismetMathLibrary.Normal` (- _targetlocation _returnvalue)) 1500.0)))))
  (bind (_returnvalue_roll_2 _returnvalue_pitch_2 _returnvalue_yaw_2) (`KismetMathLibrary.BreakRotator` (`KismetMathLibrary.RInterpTo` _returnvalue_2 (`KismetMathLibrary.MakeRotator` _returnvalue_roll _returnvalue_pitch _returnvalue_yaw) DeltaSeconds 2.0)))
  (if (and (not (`self.PeixeTipo1`)) (not (`self.PeixeTipo2`)))
    (`self.3ºPeixe`)
    (else
      (if (and (`self.PeixeTipo1`) (not (`self.PeixeTipo2`)))
        (if (`self.CanMoveAgain`)
          (`self.MoveAway`)))
      (bind _returnvalue_3 (`GameplayStatics.GetActorOfClass` "/Game/KillYourBabiesBPS/BP_PLayer/BP_ThirdPersonCharacterKYB.BP_ThirdPersonCharacterKYB_C"))
      (bind _returnvalue_4 (`GameplayStatics.GetActorOfClass` "/Game/KillYourBabiesBPS/BPS_Foca/FocaTentativa.FocaTentativa_C"))
      (bind _returnvalue_5 (`GameplayStatics.GetActorOfClass` "/Game/KillYourBabiesBPS/BPS_Foca/FocaNavPointFollow.FocaNavPointFollow_C"))
      (if (`/Game/KillYourBabiesBPS/BPS_Foca/FocaNavPointFollow.IsFollowing` _returnvalue_5)
        (bind (_returnvalue_roll_3 _returnvalue_pitch_3 _returnvalue_yaw_3) (`KismetMathLibrary.BreakRotator` (`KismetMathLibrary.RInterpTo` (`SceneComponent.K2_GetComponentRotation` _peixe) (`KismetMathLibrary.FindLookAtRotation` (`SceneComponent.K2_GetComponentLocation` _peixe) (`SceneComponent.K2_GetComponentLocation` (`/Game/KillYourBabiesBPS/BPS_Foca/FocaTentativa.SkeletalMesh` _returnvalue_4))) DeltaSeconds 6.0)))
        (`SceneComponent.K2_SetWorldRotation` _defaultsceneroot (`KismetMathLibrary.MakeRotator` _returnvalue_roll_3 _returnvalue_pitch_3 _returnvalue_yaw_3) false false)
        (else
          (bind _returnvalue_6 (`SceneComponent.K2_GetComponentLocation` (`/Game/KillYourBabiesBPS/BP_PLayer/BP_ThirdPersonCharacterKYB.SkeletalMesh` _returnvalue_3)))
          (if (and (and (not (`self.PeixeTipo1`)) (`self.PeixeTipo2`)) (< (`KismetMathLibrary.Vector_Distance` _returnvalue _returnvalue_6) 1500.0))
            (bind (_returnvalue_roll_4 _returnvalue_pitch_4 _returnvalue_yaw_4) (`KismetMathLibrary.BreakRotator` (`KismetMathLibrary.FindLookAtRotation` _returnvalue _returnvalue_6)))
            (bind (_returnvalue_roll_5 _returnvalue_pitch_5 _returnvalue_yaw_5) (`KismetMathLibrary.BreakRotator` (`KismetMathLibrary.RInterpTo` _returnvalue_2 (`KismetMathLibrary.MakeRotator` _returnvalue_roll_4 _returnvalue_pitch_4 _returnvalue_yaw_4) DeltaSeconds 6.0)))
            (`SceneComponent.K2_SetWorldRotation` _defaultsceneroot (`KismetMathLibrary.MakeRotator` _returnvalue_roll_5 _returnvalue_pitch_5 _returnvalue_yaw_5) false false)
            (else
              (`KismetSystemLibrary.PrintString` (`KismetStringLibrary.Conv_VectorToString` _targetlocation))
              (`SceneComponent.K2_SetWorldRotation` _defaultsceneroot (`KismetMathLibrary.MakeRotator` _returnvalue_roll_2 _returnvalue_pitch_2 _returnvalue_yaw_2) false false))))))))

(event `self.ReceiveDestroyed`
  (`FMODBlueprintStatics.PlayEvent2D` "/Game/FMOD/Events/SFX/Collect_Fish.Collect_Fish")
  (bind _returnvalue (`GameplayStatics.GetActorOfClass` "/Game/KillYourBabiesBPS/Peixes/PeixeManager.PeixeManager_C"))
  (`BlueprintMapLibrary.Map_Remove` (`/Game/KillYourBabiesBPS/Peixes/PeixeManager.ActiveFishMap` _returnvalue) (`self.MySpawnPoint`)))

(event `ComerPeixe`
  (bind _returnvalue (`GameplayStatics.GetActorOfClass` "/Game/KillYourBabiesBPS/BP_PLayer/BP_ThirdPersonCharacterKYB.BP_ThirdPersonCharacterKYB_C"))
  (if (< (`/Game/KillYourBabiesBPS/BP_PLayer/BP_ThirdPersonCharacterKYB.Peixes` _returnvalue) (`self.MaxPeixe`))
    (if (`self.PeixeTipo1`)
      (set `/Game/KillYourBabiesBPS/BP_PLayer/BP_ThirdPersonCharacterKYB.Peixes` (+ (`/Game/KillYourBabiesBPS/BP_PLayer/BP_ThirdPersonCharacterKYB.Peixes` _returnvalue) 1.0) _returnvalue)
      (elif (`self.PeixeTipo2`)
        (set `/Game/KillYourBabiesBPS/BP_PLayer/BP_ThirdPersonCharacterKYB.Peixes` (+ (`/Game/KillYourBabiesBPS/BP_PLayer/BP_ThirdPersonCharacterKYB.Peixes` _returnvalue) 3.0) _returnvalue)
        (else
          (set `/Game/KillYourBabiesBPS/BP_PLayer/BP_ThirdPersonCharacterKYB.Peixes` (+ (`/Game/KillYourBabiesBPS/BP_PLayer/BP_ThirdPersonCharacterKYB.Peixes` _returnvalue) 5.0) _returnvalue))))
    (bind _returnvalue_2 (`GameplayStatics.GetActorOfClass` "/Game/KillYourBabiesBPS/Peixes/PeixeManager.PeixeManager_C"))
    (`/Game/KillYourBabiesBPS/Peixes/PeixeManager.SpawnFishAtPoint` _returnvalue_2)
    (`KismetSystemLibrary.PrintString` "Hello")
    (`self.K2_DestroyActor` self)))

(event `PeixeUpdate`
  (bind _returnvalue (`GameplayStatics.GetActorOfClass` "/Game/KillYourBabiesBPS/BP_PLayer/BP_ThirdPersonCharacterKYB.BP_ThirdPersonCharacterKYB_C"))
  (if (`/Game/KillYourBabiesBPS/BP_PLayer/BP_ThirdPersonCharacterKYB.Has0PenguinReady` _returnvalue)
    (set `self.MaxPeixe` 2.0)
    (bind _returnvalue_2 (`GameplayStatics.GetActorOfClass` "/Game/KillYourBabiesBPS/BP_PLayer/BP_ThirdPersonCharacterKYB.BP_ThirdPersonCharacterKYB_C"))
    (bind _cameraboom (`HuddleCharacter.CameraBoom` _returnvalue_2))
    (set `SpringArmComponent.TargetArmLength` (`KismetMathLibrary.Lerp` (`SpringArmComponent.TargetArmLength` _cameraboom) 650.0 0.02) _cameraboom)
    (`self.PenguinPositions0`)
    (elif (`/Game/KillYourBabiesBPS/BP_PLayer/BP_ThirdPersonCharacterKYB.Has1PenguinReady` _returnvalue)
      (set `self.MaxPeixe` 4.0)
      (bind _returnvalue_3 (`GameplayStatics.GetActorOfClass` "/Game/KillYourBabiesBPS/BP_PLayer/BP_ThirdPersonCharacterKYB.BP_ThirdPersonCharacterKYB_C"))
      (bind _cameraboom_2 (`HuddleCharacter.CameraBoom` _returnvalue_3))
      (set `SpringArmComponent.TargetArmLength` (`KismetMathLibrary.Lerp` (`SpringArmComponent.TargetArmLength` _cameraboom_2) 700.0 0.02) _cameraboom_2)
      (`self.PenguinPositions1`)
      (elif (`/Game/KillYourBabiesBPS/BP_PLayer/BP_ThirdPersonCharacterKYB.Has2PenguinReady` _returnvalue)
        (set `self.MaxPeixe` 6.0)
        (bind _returnvalue_4 (`GameplayStatics.GetActorOfClass` "/Game/KillYourBabiesBPS/BP_PLayer/BP_ThirdPersonCharacterKYB.BP_ThirdPersonCharacterKYB_C"))
        (bind _cameraboom_3 (`HuddleCharacter.CameraBoom` _returnvalue_4))
        (set `SpringArmComponent.TargetArmLength` (`KismetMathLibrary.Lerp` (`SpringArmComponent.TargetArmLength` _cameraboom_3) 800.0 0.02) _cameraboom_3)
        (`self.PenguinPositions2`)
        (elif (`/Game/KillYourBabiesBPS/BP_PLayer/BP_ThirdPersonCharacterKYB.Has3PenguinReady` _returnvalue)
          (set `self.MaxPeixe` 8.0)
          (bind _returnvalue_5 (`GameplayStatics.GetActorOfClass` "/Game/KillYourBabiesBPS/BP_PLayer/BP_ThirdPersonCharacterKYB.BP_ThirdPersonCharacterKYB_C"))
          (bind _cameraboom_4 (`HuddleCharacter.CameraBoom` _returnvalue_5))
          (set `SpringArmComponent.TargetArmLength` (`KismetMathLibrary.Lerp` (`SpringArmComponent.TargetArmLength` _cameraboom_4) 900.0 0.02) _cameraboom_4)
          (`self.PenguinPositions3`)
          (elif (`/Game/KillYourBabiesBPS/BP_PLayer/BP_ThirdPersonCharacterKYB.Has4PenguinReady` _returnvalue)
            (set `self.MaxPeixe` 10.0)
            (bind _returnvalue_6 (`GameplayStatics.GetActorOfClass` "/Game/KillYourBabiesBPS/BP_PLayer/BP_ThirdPersonCharacterKYB.BP_ThirdPersonCharacterKYB_C"))
            (bind _cameraboom_5 (`HuddleCharacter.CameraBoom` _returnvalue_6))
            (set `SpringArmComponent.TargetArmLength` (`KismetMathLibrary.Lerp` (`SpringArmComponent.TargetArmLength` _cameraboom_5) 1000.0 0.02) _cameraboom_5)
            (`self.PenguinPositions4`)))))))

(fn `PenguinPositions0`
  (bind _returnvalue (`GameplayStatics.GetActorOfClass` "/Game/KillYourBabiesBPS/BP_PLayer/BP_ThirdPersonCharacterKYB.BP_ThirdPersonCharacterKYB_C"))
  (bind _skeletalmesh (`/Game/KillYourBabiesBPS/BP_PLayer/BP_ThirdPersonCharacterKYB.SkeletalMesh` _returnvalue))
  (bind _output_get (set `/Game/KillYourBabiesBPS/BP_PLayer/BP_ThirdPersonCharacterKYB.OriginalLocation_0` (`KismetMathLibrary.VLerp` (`SceneComponent.RelativeLocation` _skeletalmesh) (74.378734 48.315798 -164.002911) (`self.AdjustingSpeed`)) _returnvalue))
  (set `/Game/KillYourBabiesBPS/BP_PLayer/BP_ThirdPersonCharacterKYB.AmplitudeX_0` 1.0 _returnvalue)
  (set `/Game/KillYourBabiesBPS/BP_PLayer/BP_ThirdPersonCharacterKYB.AmplitudeY_0` 1.0 _returnvalue)
  (set `/Game/KillYourBabiesBPS/BP_PLayer/BP_ThirdPersonCharacterKYB.AmplitudeZ_0` 1.0 _returnvalue)
  (`SceneComponent.K2_SetRelativeLocation` _skeletalmesh _output_get false false))

(fn `PenguinPositions1`
  (bind _returnvalue (`GameplayStatics.GetActorOfClass` "/Game/KillYourBabiesBPS/BP_PLayer/BP_ThirdPersonCharacterKYB.BP_ThirdPersonCharacterKYB_C"))
  (bind _skeletalmesh (`/Game/KillYourBabiesBPS/BP_PLayer/BP_ThirdPersonCharacterKYB.SkeletalMesh` _returnvalue))
  (bind _output_get (set `/Game/KillYourBabiesBPS/BP_PLayer/BP_ThirdPersonCharacterKYB.OriginalLocation_0` (`KismetMathLibrary.VLerp` (`SceneComponent.RelativeLocation` _skeletalmesh) (-23.72205 -113.605215 -164.002913) (`self.AdjustingSpeed`)) _returnvalue))
  (set `/Game/KillYourBabiesBPS/BP_PLayer/BP_ThirdPersonCharacterKYB.AmplitudeX_0` 1.0 _returnvalue)
  (set `/Game/KillYourBabiesBPS/BP_PLayer/BP_ThirdPersonCharacterKYB.AmplitudeY_0` 1.0 _returnvalue)
  (set `/Game/KillYourBabiesBPS/BP_PLayer/BP_ThirdPersonCharacterKYB.AmplitudeZ_0` 1.0 _returnvalue)
  (`SceneComponent.K2_SetRelativeLocation` _skeletalmesh _output_get false false)
  (bind _returnvalue_2 (`GameplayStatics.GetActorOfClass` "/Game/KillYourBabiesBPS/Penguins/NaturalMovementManager.NaturalMovementManager_C"))
  (bind _penguin1 (`/Game/KillYourBabiesBPS/BP_PLayer/BP_ThirdPersonCharacterKYB.Penguin1` _returnvalue))
  (bind _output_get_2 (set `/Game/KillYourBabiesBPS/Penguins/NaturalMovementManager.OriginalLocation_1` (`KismetMathLibrary.VLerp` (`SceneComponent.RelativeLocation` _penguin1) (-10.659666 162.889961 -47.198271) (`self.AdjustingSpeed`)) _returnvalue_2))
  (set `/Game/KillYourBabiesBPS/Penguins/NaturalMovementManager.AmplitudeX_1` 1.0 _returnvalue_2)
  (set `/Game/KillYourBabiesBPS/Penguins/NaturalMovementManager.AmplitudeY_1` 1.0 _returnvalue_2)
  (set `/Game/KillYourBabiesBPS/Penguins/NaturalMovementManager.AmplitudeZ_1` 1.0 _returnvalue_2)
  (`SceneComponent.K2_SetRelativeLocation` _penguin1 _output_get_2 false false))

(fn `PenguinPositions2`
  (bind _returnvalue (`GameplayStatics.GetActorOfClass` "/Game/KillYourBabiesBPS/BP_PLayer/BP_ThirdPersonCharacterKYB.BP_ThirdPersonCharacterKYB_C"))
  (bind _skeletalmesh (`/Game/KillYourBabiesBPS/BP_PLayer/BP_ThirdPersonCharacterKYB.SkeletalMesh` _returnvalue))
  (bind _output_get (set `/Game/KillYourBabiesBPS/BP_PLayer/BP_ThirdPersonCharacterKYB.OriginalLocation_0` (`KismetMathLibrary.VLerp` (`SceneComponent.RelativeLocation` _skeletalmesh) (-23.72205 -113.605215 -174.002913) (`self.AdjustingSpeed`)) _returnvalue))
  (set `/Game/KillYourBabiesBPS/BP_PLayer/BP_ThirdPersonCharacterKYB.AmplitudeX_0` 1.0 _returnvalue)
  (set `/Game/KillYourBabiesBPS/BP_PLayer/BP_ThirdPersonCharacterKYB.AmplitudeY_0` 1.0 _returnvalue)
  (set `/Game/KillYourBabiesBPS/BP_PLayer/BP_ThirdPersonCharacterKYB.AmplitudeZ_0` 1.0 _returnvalue)
  (`SceneComponent.K2_SetRelativeLocation` _skeletalmesh _output_get false false)
  (bind _returnvalue_2 (`GameplayStatics.GetActorOfClass` "/Game/KillYourBabiesBPS/Penguins/NaturalMovementManager.NaturalMovementManager_C"))
  (bind _penguin1 (`/Game/KillYourBabiesBPS/BP_PLayer/BP_ThirdPersonCharacterKYB.Penguin1` _returnvalue))
  (bind _output_get_2 (set `/Game/KillYourBabiesBPS/Penguins/NaturalMovementManager.OriginalLocation_1` (`KismetMathLibrary.VLerp` (`SceneComponent.RelativeLocation` _penguin1) (-111.757224 39.318341 -87.365358) (`self.AdjustingSpeed`)) _returnvalue_2))
  (set `/Game/KillYourBabiesBPS/Penguins/NaturalMovementManager.AmplitudeX_1` 1.0 _returnvalue_2)
  (set `/Game/KillYourBabiesBPS/Penguins/NaturalMovementManager.AmplitudeY_1` 1.0 _returnvalue_2)
  (set `/Game/KillYourBabiesBPS/Penguins/NaturalMovementManager.AmplitudeZ_1` 1.0 _returnvalue_2)
  (`SceneComponent.K2_SetRelativeLocation` _penguin1 _output_get_2 false false)
  (bind _returnvalue_3 (`GameplayStatics.GetActorOfClass` "/Game/KillYourBabiesBPS/Penguins/NaturalMovementManager.NaturalMovementManager_C"))
  (bind _penguin2 (`/Game/KillYourBabiesBPS/BP_PLayer/BP_ThirdPersonCharacterKYB.Penguin2` _returnvalue))
  (bind _output_get_3 (set `/Game/KillYourBabiesBPS/Penguins/NaturalMovementManager.OriginalLocation_2` (`KismetMathLibrary.VLerp` (`SceneComponent.RelativeLocation` _penguin2) (-10.659666 162.889961 -47.198271) (`self.AdjustingSpeed`)) _returnvalue_3))
  (set `/Game/KillYourBabiesBPS/Penguins/NaturalMovementManager.AmplitudeX_2` 1.0 _returnvalue_3)
  (set `/Game/KillYourBabiesBPS/Penguins/NaturalMovementManager.AmplitudeY_2` 1.0 _returnvalue_3)
  (set `/Game/KillYourBabiesBPS/Penguins/NaturalMovementManager.AmplitudeZ_2` 1.0 _returnvalue_3)
  (`SceneComponent.K2_SetRelativeLocation` _penguin2 _output_get_3 false false))

(fn `PenguinPositions3`
  (bind _returnvalue (`GameplayStatics.GetActorOfClass` "/Game/KillYourBabiesBPS/BP_PLayer/BP_ThirdPersonCharacterKYB.BP_ThirdPersonCharacterKYB_C"))
  (bind _skeletalmesh (`/Game/KillYourBabiesBPS/BP_PLayer/BP_ThirdPersonCharacterKYB.SkeletalMesh` _returnvalue))
  (bind _output_get (set `/Game/KillYourBabiesBPS/BP_PLayer/BP_ThirdPersonCharacterKYB.OriginalLocation_0` (`KismetMathLibrary.VLerp` (`SceneComponent.RelativeLocation` _skeletalmesh) (3.86 -104.54 -180.0) (`self.AdjustingSpeed`)) _returnvalue))
  (set `/Game/KillYourBabiesBPS/BP_PLayer/BP_ThirdPersonCharacterKYB.AmplitudeX_0` 1.0 _returnvalue)
  (set `/Game/KillYourBabiesBPS/BP_PLayer/BP_ThirdPersonCharacterKYB.AmplitudeY_0` 1.0 _returnvalue)
  (set `/Game/KillYourBabiesBPS/BP_PLayer/BP_ThirdPersonCharacterKYB.AmplitudeZ_0` 1.0 _returnvalue)
  (`SceneComponent.K2_SetRelativeLocation` _skeletalmesh _output_get false false)
  (bind _returnvalue_2 (`GameplayStatics.GetActorOfClass` "/Game/KillYourBabiesBPS/Penguins/NaturalMovementManager.NaturalMovementManager_C"))
  (bind _penguin1 (`/Game/KillYourBabiesBPS/BP_PLayer/BP_ThirdPersonCharacterKYB.Penguin1` _returnvalue))
  (bind _output_get_2 (set `/Game/KillYourBabiesBPS/Penguins/NaturalMovementManager.OriginalLocation_1` (`KismetMathLibrary.VLerp` (`SceneComponent.RelativeLocation` _penguin1) (17.8 176.5 -96.3) (`self.AdjustingSpeed`)) _returnvalue_2))
  (set `/Game/KillYourBabiesBPS/Penguins/NaturalMovementManager.AmplitudeX_1` 1.0 _returnvalue_2)
  (set `/Game/KillYourBabiesBPS/Penguins/NaturalMovementManager.AmplitudeY_1` 1.0 _returnvalue_2)
  (set `/Game/KillYourBabiesBPS/Penguins/NaturalMovementManager.AmplitudeZ_1` 1.0 _returnvalue_2)
  (`SceneComponent.K2_SetRelativeLocation` _penguin1 _output_get_2 false false)
  (bind _returnvalue_3 (`GameplayStatics.GetActorOfClass` "/Game/KillYourBabiesBPS/Penguins/NaturalMovementManager.NaturalMovementManager_C"))
  (bind _penguin2 (`/Game/KillYourBabiesBPS/BP_PLayer/BP_ThirdPersonCharacterKYB.Penguin2` _returnvalue))
  (bind _output_get_3 (set `/Game/KillYourBabiesBPS/Penguins/NaturalMovementManager.OriginalLocation_2` (`KismetMathLibrary.VLerp` (`SceneComponent.RelativeLocation` _penguin2) (-117.2 38.5 -82.5) (`self.AdjustingSpeed`)) _returnvalue_3))
  (set `/Game/KillYourBabiesBPS/Penguins/NaturalMovementManager.AmplitudeX_2` 1.0 _returnvalue_3)
  (set `/Game/KillYourBabiesBPS/Penguins/NaturalMovementManager.AmplitudeY_2` 1.0 _returnvalue_3)
  (set `/Game/KillYourBabiesBPS/Penguins/NaturalMovementManager.AmplitudeZ_2` 1.0 _returnvalue_3)
  (`SceneComponent.K2_SetRelativeLocation` _penguin2 _output_get_3 false false)
  (bind _returnvalue_4 (`GameplayStatics.GetActorOfClass` "/Game/KillYourBabiesBPS/Penguins/NaturalMovementManager.NaturalMovementManager_C"))
  (bind _penguin3 (`/Game/KillYourBabiesBPS/BP_PLayer/BP_ThirdPersonCharacterKYB.Penguin3` _returnvalue))
  (bind _output_get_4 (set `/Game/KillYourBabiesBPS/Penguins/NaturalMovementManager.OriginalLocation_3` (`KismetMathLibrary.VLerp` (`SceneComponent.RelativeLocation` _penguin3) (140.1 28.92 -61.0) (`self.AdjustingSpeed`)) _returnvalue_4))
  (set `/Game/KillYourBabiesBPS/Penguins/NaturalMovementManager.AmplitudeX_3` 1.0 _returnvalue_4)
  (set `/Game/KillYourBabiesBPS/Penguins/NaturalMovementManager.AmplitudeY_3` 1.0 _returnvalue_4)
  (set `/Game/KillYourBabiesBPS/Penguins/NaturalMovementManager.AmplitudeZ_3` 1.0 _returnvalue_4)
  (`SceneComponent.K2_SetRelativeLocation` _penguin3 _output_get_4 false false))

(fn `PenguinPositions4`
  (bind _returnvalue (`GameplayStatics.GetActorOfClass` "/Game/KillYourBabiesBPS/BP_PLayer/BP_ThirdPersonCharacterKYB.BP_ThirdPersonCharacterKYB_C"))
  (bind _skeletalmesh (`/Game/KillYourBabiesBPS/BP_PLayer/BP_ThirdPersonCharacterKYB.SkeletalMesh` _returnvalue))
  (bind _output_get (set `/Game/KillYourBabiesBPS/BP_PLayer/BP_ThirdPersonCharacterKYB.OriginalLocation_0` (`KismetMathLibrary.VLerp` (`SceneComponent.RelativeLocation` _skeletalmesh) (19.91 -130.14 -42.132) (`self.AdjustingSpeed`)) _returnvalue))
  (set `/Game/KillYourBabiesBPS/BP_PLayer/BP_ThirdPersonCharacterKYB.AmplitudeX_0` 1.0 _returnvalue)
  (set `/Game/KillYourBabiesBPS/BP_PLayer/BP_ThirdPersonCharacterKYB.AmplitudeY_0` 1.0 _returnvalue)
  (set `/Game/KillYourBabiesBPS/BP_PLayer/BP_ThirdPersonCharacterKYB.AmplitudeZ_0` 1.0 _returnvalue)
  (`SceneComponent.K2_SetRelativeLocation` _skeletalmesh _output_get false false)
  (bind _returnvalue_2 (`GameplayStatics.GetActorOfClass` "/Game/KillYourBabiesBPS/Penguins/NaturalMovementManager.NaturalMovementManager_C"))
  (bind _penguin1 (`/Game/KillYourBabiesBPS/BP_PLayer/BP_ThirdPersonCharacterKYB.Penguin1` _returnvalue))
  (bind _output_get_2 (set `/Game/KillYourBabiesBPS/Penguins/NaturalMovementManager.OriginalLocation_1` (`KismetMathLibrary.VLerp` (`SceneComponent.RelativeLocation` _penguin1) (4.25 165.66 -94.387) (`self.AdjustingSpeed`)) _returnvalue_2))
  (set `/Game/KillYourBabiesBPS/Penguins/NaturalMovementManager.AmplitudeX_1` 1.0 _returnvalue_2)
  (set `/Game/KillYourBabiesBPS/Penguins/NaturalMovementManager.AmplitudeY_1` 1.0 _returnvalue_2)
  (set `/Game/KillYourBabiesBPS/Penguins/NaturalMovementManager.AmplitudeZ_1` 1.0 _returnvalue_2)
  (`SceneComponent.K2_SetRelativeLocation` _penguin1 _output_get_2 false false)
  (bind _returnvalue_3 (`GameplayStatics.GetActorOfClass` "/Game/KillYourBabiesBPS/Penguins/NaturalMovementManager.NaturalMovementManager_C"))
  (bind _penguin2 (`/Game/KillYourBabiesBPS/BP_PLayer/BP_ThirdPersonCharacterKYB.Penguin2` _returnvalue))
  (bind _output_get_3 (set `/Game/KillYourBabiesBPS/Penguins/NaturalMovementManager.OriginalLocation_2` (`KismetMathLibrary.VLerp` (`SceneComponent.RelativeLocation` _penguin2) (-21.71 -90.283 -95.049) (`self.AdjustingSpeed`)) _returnvalue_3))
  (set `/Game/KillYourBabiesBPS/Penguins/NaturalMovementManager.AmplitudeX_2` 1.0 _returnvalue_3)
  (set `/Game/KillYourBabiesBPS/Penguins/NaturalMovementManager.AmplitudeY_2` 1.0 _returnvalue_3)
  (set `/Game/KillYourBabiesBPS/Penguins/NaturalMovementManager.AmplitudeZ_2` 1.0 _returnvalue_3)
  (`SceneComponent.K2_SetRelativeLocation` _penguin2 _output_get_3 false false)
  (bind _returnvalue_4 (`GameplayStatics.GetActorOfClass` "/Game/KillYourBabiesBPS/Penguins/NaturalMovementManager.NaturalMovementManager_C"))
  (bind _penguin3 (`/Game/KillYourBabiesBPS/BP_PLayer/BP_ThirdPersonCharacterKYB.Penguin3` _returnvalue))
  (bind _output_get_4 (set `/Game/KillYourBabiesBPS/Penguins/NaturalMovementManager.OriginalLocation_3` (`KismetMathLibrary.VLerp` (`SceneComponent.RelativeLocation` _penguin3) (141.655 28.92 -50.007) (`self.AdjustingSpeed`)) _returnvalue_4))
  (set `/Game/KillYourBabiesBPS/Penguins/NaturalMovementManager.AmplitudeX_3` 1.0 _returnvalue_4)
  (set `/Game/KillYourBabiesBPS/Penguins/NaturalMovementManager.AmplitudeY_3` 1.0 _returnvalue_4)
  (set `/Game/KillYourBabiesBPS/Penguins/NaturalMovementManager.AmplitudeZ_3` 1.0 _returnvalue_4)
  (`SceneComponent.K2_SetRelativeLocation` _penguin3 _output_get_4 false false)
  (bind _returnvalue_5 (`GameplayStatics.GetActorOfClass` "/Game/KillYourBabiesBPS/Penguins/NaturalMovementManager.NaturalMovementManager_C"))
  (bind _penguin4 (`/Game/KillYourBabiesBPS/BP_PLayer/BP_ThirdPersonCharacterKYB.Penguin4` _returnvalue))
  (bind _output_get_5 (set `/Game/KillYourBabiesBPS/Penguins/NaturalMovementManager.OriginalLocation_4` (`KismetMathLibrary.VLerp` (`SceneComponent.RelativeLocation` _penguin4) (-39.179 190.0 55.0) (`self.AdjustingSpeed`)) _returnvalue_5))
  (set `/Game/KillYourBabiesBPS/Penguins/NaturalMovementManager.AmplitudeX_4` 1.0 _returnvalue_5)
  (set `/Game/KillYourBabiesBPS/Penguins/NaturalMovementManager.AmplitudeY_4` 1.0 _returnvalue_5)
  (set `/Game/KillYourBabiesBPS/Penguins/NaturalMovementManager.AmplitudeZ_4` 1.0 _returnvalue_5)
  (`SceneComponent.K2_SetRelativeLocation` _penguin4 _output_get_5 false false))

(fn `UserConstructionScript`)