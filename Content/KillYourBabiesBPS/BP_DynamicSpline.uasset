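; BP_DynamicSpline is an actor that records the path of BP_ThirdPersonCharacterKYB into its Spline component.
; On BeginPlay it clears the spline and adds a first point at the character capsule's world location.
; Every Tick it looks the character up again with GetActorOfClass and appends another point, so the spline grows each frame with no limit or pruning.
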(event `self.ReceiveBeginPlay`
  (`SplineComponent.ClearSplinePoints` (`self.Spline`) true)
  (bind _returnvalue (`GameplayStatics.GetActorOfClass` "/Game/KillYourBabiesBPS/VersãoNormal3ªPessoa/BP_ThirdPersonCharacterKYB.BP_ThirdPersonCharacterKYB_C"))
  (bind _asbp_third_person_character_kyb (cast `/Game/KillYourBabiesBPS/VersãoNormal3ªPessoa/BP_ThirdPersonCharacterKYB` _returnvalue))
  (`SplineComponent.AddSplinePoint` (`self.Spline`) (`SceneComponent.K2_GetComponentLocation` (`Character.CapsuleComponent` _asbp_third_person_character_kyb)) "World" true))

(event `self.ReceiveTick`
  (params (DeltaSeconds :type "Float (single-precision)"))
  (bind _returnvalue (`GameplayStatics.GetActorOfClass` "/Game/KillYourBabiesBPS/VersãoNormal3ªPessoa/BP_ThirdPersonCharacterKYB.BP_ThirdPersonCharacterKYB_C"))
  (bind _asbp_third_person_character_kyb (cast `/Game/KillYourBabiesBPS/VersãoNormal3ªPessoa/BP_ThirdPersonCharacterKYB` _returnvalue))
  (`SplineComponent.AddSplinePoint` (`self.Spline`) (`SceneComponent.K2_GetComponentLocation` (`Character.CapsuleComponent` _asbp_third_person_character_kyb)) "World" true))

(fn `UserConstructionScript`)