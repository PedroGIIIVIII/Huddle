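; Actor that caps the player's fish (Peixes) count according to how many penguins are held.
; Every Tick it fetches the KYB third-person character and BP_Peixes, then checks the latter's zero, one and two penguin flags, each with a higher limit.
; When the count exceeds the matching limit, it clamps the character's value, prints a debug string and calls PeixeUpdate on BP_Peixes.
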(event `self.ReceiveTick`
  (params (DeltaSeconds :type "Float (single-precision)"))
  (bind _returnvalue (`GameplayStatics.GetActorOfClass` "/Game/KillYourBabiesBPS/VersãoNormal3ªPessoa/BP_ThirdPersonCharacterKYB.BP_ThirdPersonCharacterKYB_C"))
  (bind _returnvalue_2 (`GameplayStatics.GetActorOfClass` "/Game/KillYourBabiesBPS/Peixes/BP_Peixes.BP_Peixes_C"))
  (bind _peixes (`/Game/KillYourBabiesBPS/VersãoNormal3ªPessoa/BP_ThirdPersonCharacterKYB.Peixes` _returnvalue))
  (if (and (`/Game/KillYourBabiesBPS/Peixes/BP_Peixes.Have0Penguins` _returnvalue_2) (> _peixes 2.0))
    (set `/Game/KillYourBabiesBPS/VersãoNormal3ªPessoa/BP_ThirdPersonCharacterKYB.Peixes` 2.0 _returnvalue)
    (`KismetSystemLibrary.PrintString` "0")
    (`/Game/KillYourBabiesBPS/Peixes/BP_Peixes.PeixeUpdate` _returnvalue_2)
    (elif (and (`/Game/KillYourBabiesBPS/Peixes/BP_Peixes.Have1Penguins` _returnvalue_2) (> _peixes 4.0))
      (set `/Game/KillYourBabiesBPS/VersãoNormal3ªPessoa/BP_ThirdPersonCharacterKYB.Peixes` 4.0 _returnvalue)
      (`KismetSystemLibrary.PrintString` "1")
      (`/Game/KillYourBabiesBPS/Peixes/BP_Peixes.PeixeUpdate` _returnvalue_2)
      (elif (and (`/Game/KillYourBabiesBPS/Peixes/BP_Peixes.Have2Penguins` _returnvalue_2) (> _peixes 6.0))
        (set `/Game/KillYourBabiesBPS/VersãoNormal3ªPessoa/BP_ThirdPersonCharacterKYB.Peixes` 6.0 _returnvalue)
        (`KismetSystemLibrary.PrintString` "2")
        (`/Game/KillYourBabiesBPS/Peixes/BP_Peixes.PeixeUpdate` _returnvalue_2)))))

(fn `UserConstructionScript`)