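; BP_RainhaAnimSound plays an FMOD sound in time with the animation on the Queen_Blueprint actor.
; Each Tick it looks up the Queen, prints her skeletal mesh's playback position, and plays the audio once that passes a set threshold while CanSneeze is true.
; It clears the Queen's CanSneeze flag on playback and restores it after a fixed Delay, limiting how often the sound repeats.
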(event `self.ReceiveTick`
  (params (DeltaSeconds :type "Float (single-precision)"))
  (bind _returnvalue (`GameplayStatics.GetActorOfClass` "/Game/Assets/Models/Rigged/Queen/queen_Blueprint.queen_Blueprint_C"))
  (bind _returnvalue_2 (`SkeletalMeshComponent.GetPosition` (`SkeletalMeshActor.SkeletalMeshComponent` _returnvalue)))
  (`KismetSystemLibrary.PrintString` (`KismetStringLibrary.Conv_DoubleToString` _returnvalue_2))
  (if (and (>= _returnvalue_2 1.94) (`/Game/Assets/Models/Rigged/Queen/queen_Blueprint.CanSneeze` _returnvalue))
    (set `/Game/Assets/Models/Rigged/Queen/queen_Blueprint.CanSneeze` false _returnvalue)
    (`FMODAudioComponent.Play` (`self.FMODAudio`))
    (`KismetSystemLibrary.Delay` 19.94)
    (set `/Game/Assets/Models/Rigged/Queen/queen_Blueprint.CanSneeze` true _returnvalue)))

(fn `UserConstructionScript`)