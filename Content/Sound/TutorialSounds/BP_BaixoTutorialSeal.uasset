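; Tutorial audio actor that drives an FMOD sound, apparently a bass ("Baixo") layer, by the player's proximity.
; It raises the "Fade Long" parameter on BeginPlay and drops it while the TutorialManager's StopBaixo flag is set.
; Otherwise, Tick maps player distance against DistânciaMáxima to a clamped, inverted "Proximity" parameter.
; The manager is looked up with GetActorOfClass every frame.
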(event `self.ReceiveBeginPlay`
  (`FMODAudioComponent.SetParameter` (`self.FMODAudio`) "Fade Long" 1.0))

(event `self.ReceiveTick`
  (params (DeltaSeconds :type "Float (single-precision)"))
  (bind _returnvalue (`GameplayStatics.GetActorOfClass` "/Game/KillYourBabiesBPS/Tutorial/TutorialManager.TutorialManager_C"))
  (if (`/Game/KillYourBabiesBPS/Tutorial/TutorialManager.StopBaixo` _returnvalue)
    (`FMODAudioComponent.SetParameter` (`self.FMODAudio`) "Fade Long" 0.0)
    (else
      (`FMODAudioComponent.SetParameter` (`self.FMODAudio`) "Proximity" (`KismetMathLibrary.FClamp` (- 1.0 (/ (`KismetMathLibrary.Vector_Distance` (`SceneComponent.K2_GetComponentLocation` (`self.DefaultSceneRoot`)) (`SceneComponent.K2_GetComponentLocation` (`Character.CapsuleComponent` (`GameplayStatics.GetPlayerCharacter` 0)))) (`self.DistânciaMáxima`))))))))

(fn `UserConstructionScript`)