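; BP_TunelFoca is an AI-driven swimming seal (foca) character that patrols and chases the player on sight.
; FocaPatrol moves it through a looping set of four PatrolLocation points at a slow swim speed.
; Every Tick, a forward-vector dot product and distance check selects either FocaPatrol or the faster FocaFollow, reissuing the move and printing the state.
; FocaFollow targets the player's location projected onto the navmesh.
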(event `self.ReceiveBeginPlay`
  (`self.FocaPatrol`))

(event `FocaFollow`
  (set `CharacterMovementComponent.MaxSwimSpeed` 1200.0 (`self.CharacterMovement`))
  (`|AIMoveTo` self (`NavigationSystemV1.K2_ProjectPointToNavigation` (`self.K2_GetActorLocation` (`GameplayStatics.GetPlayerCharacter` 0)) null null (1500.0 1500.0 1500.0)) null
    (:`OnSuccess`
      (`self.FocaFollow`))))

(event `FocaPatrol`
  (set `CharacterMovementComponent.MaxSwimSpeed` 600.0 (`self.CharacterMovement`))
  (`|AIMoveTo` self (`|GetArrayItem` (`self.PatrolLocation`) (`self.Locations`)) null
    (:`OnSuccess`
      (`self.FocaPatrol`)
      (`/Engine/EditorBlueprintResources/StandardMacros.IncrementInt` (`self.Locations`)
        (:`  `
          (if (== (`self.Locations`) 4)
            (set `self.Locations` 0)))))))

(event `self.ReceiveTick`
  (params (DeltaSeconds :type "Float (single-precision)"))
  (bind _capsulecomponent (`self.CapsuleComponent`))
  (bind _returnvalue (- (`self.K2_GetActorLocation` (`GameplayStatics.GetPlayerCharacter` 0)) (`SceneComponent.RelativeLocation` _capsulecomponent)))
  (if (and (>= (`KismetMathLibrary.Dot_VectorVector` (`SceneComponent.GetForwardVector` _capsulecomponent) (`KismetMathLibrary.Normal` _returnvalue)) 0.7) (<= (`KismetMathLibrary.VSize` _returnvalue) (`self.DetectionDistance`)))
    (`self.FocaFollow`)
    (`KismetSystemLibrary.PrintString` "Detected")
    (else
      (`self.FocaPatrol`)
      (`KismetSystemLibrary.PrintString` "Patrol"))))

(fn `UserConstructionScript`)