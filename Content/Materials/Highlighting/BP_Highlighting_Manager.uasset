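; Manager actor that drives pulsing highlight effects by animating the Thickness parameter of dynamic highlight materials.
; BeginPlay creates white, red and red-balloon instances, then after a short delay sets the white one as overlay on the BP_Peixes1 skeletal mesh.
; Tick restarts white and red pulses through boolean gates, each using paired forward and reverse timelines plus a pause.
; The balloon pulse is never triggered here, and neither red instance is assigned to a mesh.
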(event `FadeWhite`
  (set `self.CanFadeWhite` false)
  (bind (_direction _newtrack_0) (`Timeline|Timeline` :!via `PlayFromStart`)
    (:`Update`
      (`MaterialInstanceDynamic.SetScalarParameterValue` (stale `self.ReceiveBeginPlay` _output_get) "Thickness" _newtrack_0))
    (:`Finished`
      (bind (_direction_2 _newtrack_0_2) (`Timeline|Timeline_0` :!via `ReverseFromEnd`)
        (:`Update`
          (`MaterialInstanceDynamic.SetScalarParameterValue` (stale `self.ReceiveBeginPlay` _output_get) "Thickness" _newtrack_0_2))
        (:`Finished`
          (`KismetSystemLibrary.Delay` 0.5)
          (set `self.CanFadeWhite` true))))))

(event `self.ReceiveBeginPlay`
  (bind _returnvalue (`KismetMaterialLibrary.CreateDynamicMaterialInstance` "/Game/Materials/Highlighting/Highlight_Material1.Highlight_Material1"))
  (bind _output_get (set `self.NovoMaterialHighlightCriadoWhite` _returnvalue))
  (bind _returnvalue_2 (`KismetMaterialLibrary.CreateDynamicMaterialInstance` "/Game/Materials/Highlighting/Highlight_Material.Highlight_Material"))
  (bind _output_get_2 (set `self.NovoMaterialHighlightCriadoRed` _returnvalue_2))
  (`GameplayStatics.GetActorOfClass` "/Game/KillYourBabiesBPS/Peixes/Os_3_Peixes/BP_Peixes1.BP_Peixes1_C")
  (bind _returnvalue_3 (`KismetMaterialLibrary.CreateDynamicMaterialInstance` "/Game/Materials/Highlighting/Highlight_Material.Highlight_Material"))
  (bind _output_get_3 (set `self.NewVarRedBalon` _returnvalue_3))
  (`KismetSystemLibrary.Delay` 1.0)
  (bind _returnvalue_4 (`GameplayStatics.GetActorOfClass` "/Game/KillYourBabiesBPS/Peixes/Os_3_Peixes/BP_Peixes1.BP_Peixes1_C"))
  (`MeshComponent.SetOverlayMaterial` (`/Game/KillYourBabiesBPS/Peixes/Os_3_Peixes/BP_Peixes1.SkeletalMesh1` _returnvalue_4) _output_get))

(event `FadeRed`
  (set `self.CanFadeRed` false)
  (bind (_direction _newtrack_0) (`Timeline|Timeline_1` :!via `PlayFromStart`)
    (:`Update`
      (`MaterialInstanceDynamic.SetScalarParameterValue` (stale `self.ReceiveBeginPlay` _output_get_2) "Thickness" _newtrack_0))
    (:`Finished`
      (bind (_direction_2 _newtrack_0_2) (`Timeline|Timeline_2` :!via `ReverseFromEnd`)
        (:`Update`
          (`MaterialInstanceDynamic.SetScalarParameterValue` (stale `self.ReceiveBeginPlay` _output_get_2) "Thickness" _newtrack_0_2))
        (:`Finished`
          (`KismetSystemLibrary.Delay` 0.5)
          (set `self.CanFadeRed` true))))))

(event `self.ReceiveTick`
  (params (DeltaSeconds :type "Float (single-precision)"))
  (if (`self.CanFadeWhite`)
    (`self.FadeWhite`))
  (if (`self.CanFadeRed`)
    (`self.FadeRed`)))

(event `FadeBallonRed`
  (set `self.CanFadeBallonRed` false)
  (bind (_direction _newtrack_0) (`Timeline|Timeline_3` :!via `PlayFromStart`)
    (:`Update`
      (`MaterialInstanceDynamic.SetScalarParameterValue` (stale `self.ReceiveBeginPlay` _output_get_3) "Thickness" _newtrack_0)
      (bind (_direction_2 _newtrack_0_2) (`Timeline|Timeline_4` :!via `ReverseFromEnd`)
        (:`Update`
          (`MaterialInstanceDynamic.SetScalarParameterValue` (stale `self.ReceiveBeginPlay` _output_get_3) "Thickness" _newtrack_0_2))
        (:`Finished`
          (set `self.CanFadeBallonRed` true))))))

(fn `UserConstructionScript`)